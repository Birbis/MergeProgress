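; Test grid Blueprint that lays out child actor tiles in its construction script.
; BuildGrid loops over GridSizeA and adds a child actor component per cell, spaced by the Size default of SquareClass.
; An unused BuildHexGrid offsets alternate rows by half a column with hardcoded spacing and explicitly assigns SquareClass to each component.
; The event graph holds only disabled placeholder events.
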(event EventBeginPlay)

(event Collision|EventActorBeginOverlap
  (params (OtherActor :type Actor%20Object%20Reference)))

(event EventTick
  (params (DeltaSeconds :type Float%20%28single-precision%29)))

(fn ConstructionScript
  (CallFunction|BuildGrid))

(fn BuildGrid
  (bind _gridsizea (Variables|Default|GetGridSizeA))
  (bind _squareclass (Variables|Default|GetSquareClass))
  (bind (_x _y) (Math|Vector2D|BreakVector2D _gridsizea))
  (bind _size (Utilities|GetClassDefaults _squareclass))
  (bind _returnvalue (+ _size 0.0))
  (for _index (range 0 (Math|Float|Truncate (- _x 1.0)))
    (for _index_2 (range 0 (Math|Float|Truncate (- _y 1.0)))
      (AddComponent|AddChildActorComponent false (Math|Transform|MakeTransform (Math|Vector|MakeVector (* _index _returnvalue) (* _index_2 _returnvalue) 0.0))))))

(fn BuildHexGrid
  (for _index (range 1 (Variables|Default|GetGridSize1))
    (for _index_2 (range 1 (Variables|Default|GetGridSize2))
      (Utilities|FlowControl|Sequence
        (:then_0
          (if (> (Math|Integer|%(Integer) _index_2 2) 0)
            (Variables|Default|SetGridPositionAB (Math|Vector2D|MakeVector2D (- 0.0 (* _index_2 1.7e+03)) (+ 0.0 (* _index 2e+03))))
            (else
              (Variables|Default|SetGridPositionAB (Math|Vector2D|MakeVector2D (- 0.0 (* _index_2 1.7e+03)) (+ 1e+03 (* _index 2e+03)))))))
        (:then_1
          (bind _returnvalue (AddComponent|AddChildActorComponent false (Math|Conversions|ToTransform(Vector) (Math|Vector|MakeVector (.X (Math|Vector2D|BreakVector2D (Variables|Default|GetGridPositionAB))) (.Y (Math|Vector2D|BreakVector2D (Variables|Default|GetGridPositionAB))) 0.0))))
          (ChildActorComponent|SetChildActorClass _returnvalue (Variables|Default|GetSquareClass)))))))