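; Test player controller that lets the player touch-drag units between board squares.
; While focusing, Tick traces under the finger and sphere-traces for a BP_Test_Square, picking up the unit on the first occupied one focused.
; The dragged unit interpolates toward the finger, or toward the focused square with SnapMove.
; Releasing eases it onto an empty square, or back to its origin if the target is occupied or missing.
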(event Custom|InvalidMove
  (Components|MoveComponentTo (Variables|/Script/Engine.Actor|GetRootComponent (Variables|Default|GetMovingUnit)) (+ (Transformation|GetActorLocation (Variables|Default|GetInitialMovingSquare)) "0, 0,50.000000") "0, 0, 0" true false (Variables|Default|GetFinalMoveDuration) false)
  (Utilities|IsValid (CallFunction|GetFocusedSquare)
    (:Is%20Valid
      _)
    (:Is%20Not%20Valid
      (Default|SetFocused (Variables|Default|GetMovingUnit) false)))
  (Variables|Default|SetMovingUnit 0)
  (Variables|Default|SetbDragging false)
  (Variables|Default|SetbHolding false))

(event Custom|FinalStopMove
  (Components|MoveComponentTo (Variables|/Script/Engine.Actor|GetRootComponent (Variables|Default|GetMovingUnit)) (+ (Transformation|GetActorLocation (Variables|Default|GetLastFocusedSquare)) "0, 0,50.000000") "0, 0, 0" true false (Variables|Default|GetFinalMoveDuration) false)
  (Utilities|IsValid (CallFunction|GetFocusedSquare)
    (:Is%20Valid
      _)
    (:Is%20Not%20Valid
      (Default|SetFocused (Variables|Default|GetMovingUnit) false)))
  (Variables|Default|SetMovingUnit 0)
  (Variables|Default|SetbDragging false)
  (Variables|Default|SetbHolding false))

(event EventBeginPlay)

(event EventTick
  (params (DeltaSeconds :type Float%20%28single-precision%29))
  (|CallParentFunction DeltaSeconds)
  (CallFunction|FindFocusedSquare)
  (CallFunction|UpdateDraggedUnitLocation))

(event Input|TouchEvents|InputTouch
  (params (Location :type Vector) (FingerIndex :type ETouchIndex%20Enum))
  (:Pressed
    (CallFunction|UnfocusSquare)
    (Variables|Default|SetbFocusing true))
  (:Released
    (if (not (not (Variables|Default|GetbDragging)))
      (if (not (Variables|Default|GetbHolding))
        (CallFunction|StopHolding)
        (Variables|Default|SetbFocusing false)))))

(fn ConstructionScript)

(fn FindFocusedSquare
  (if (Variables|Default|GetbFocusing)
    (bind _output_get (Variables|Default|SetFingerLocation (.Location (Collision|BreakHitResult (.HitResult (Class|PlayerController|GetHitResultUnderFingerbyChannel "Touch1" "TraceTypeQuery3" (.bIsCurrentlyPressed (Class|PlayerController|GetInputTouchState (Variables|Default|GetFinger%20Index_0)))))))))
    (bind _outhits (Collision|MultiSphereTraceByChannel _output_get (+ _output_get "0, 0,50.000000") 5.0 "TraceTypeQuery4" false 0 "ForOneFrame"))
    (Utilities|IsValid (.HitActor (Collision|BreakHitResult (Utilities|Array|Get(acopy) _outhits)))
      (:Is%20Valid
        (bind _asbp_test_square (Utilities|Casting|CastToBP_Test_Square (.HitActor (Collision|BreakHitResult (Utilities|Array|Get(acopy) _outhits))))
          (:then
            (if (!= _asbp_test_square (Variables|Default|GetFocusedSquare))
              (CallFunction|UnfocusSquare)
              (CallFunction|SetFocusedSquare _asbp_test_square)
              (else
                (Rendering|Debug|DrawDebugPoint (Transformation|GetActorLocation _asbp_test_square) 1e+01 "(R=1.000000,G=0.402425,B=0.000000,A=1.000000)" 0.0))))
          (:CastFailed
            (CallFunction|UnfocusSquare :!label _label))))
      (:Is%20Not%20Valid
        (goto _label)))))

(fn SetFocusedSquare
  (params (Square :type BP%20Test%20Square%20Object%20Reference))
  (bind _returnvalue (CallFunction|GetFocusedSquare))
  (Variables|Default|SetFocusedSquare Square)
  (if (not (Variables|Default|GetbDragging))
    (Utilities|IsThereUnitinFocusedSquare
      (:Valid
        (Default|SetFocused (CallFunction|GetUnitinSquare) true)
        (Variables|Default|SetMovingUnit (CallFunction|GetUnitinSquare))
        (Variables|Default|SetbDragging true)
        (Default|SetDragState (CallFunction|GetMovingUnit) true)
        (Variables|Default|SetInitialMovingSquare _returnvalue)
        (Variables|/Game/Test/Blueprint/Level/BP_Test_Square.BP_Test_Square_C|SetHostedUnit _returnvalue 0)))))

(fn UnfocusSquare
  (Utilities|IsValid (CallFunction|GetFocusedSquare)
    (:Is%20Valid
      (if (not (Variables|Default|GetbDragging))
        (Utilities|IsThereUnitinFocusedSquare
          (:Valid
            (Default|SetFocused (CallFunction|GetUnitinSquare) false))
          (:Invalid
            _))))
    (:Is%20Not%20Valid
      _))
  (Utilities|IsValid (Variables|Default|GetFocusedSquare)
    (:Is%20Valid
      (Variables|Default|SetLastFocusedSquare (Variables|Default|GetFocusedSquare)))
    (:Is%20Not%20Valid
      _))
  (Variables|Default|SetFocusedSquare 0))

(fn GetFocusedSquare
  (return (Variables|Default|GetFocusedSquare)))

(fn StartDragging
  (bind _returnvalue (CallFunction|GetFocusedSquare))
  (Variables|Default|SetMovingUnit (CallFunction|GetUnitinSquare))
  (Variables|Default|SetbDragging true)
  (Default|SetDragState (CallFunction|GetMovingUnit) true)
  (Variables|Default|SetInitialMovingSquare _returnvalue)
  (Variables|/Game/Test/Blueprint/Level/BP_Test_Square.BP_Test_Square_C|SetHostedUnit _returnvalue 0))

(fn StopDragging
  (bind _returnvalue (CallFunction|GetFocusedSquare))
  (Utilities|IsValid _returnvalue
    (:Is%20Valid
      (Variables|Default|SetLastFocusedSquare _returnvalue)
      (Utilities|IsThereUnitinFocusedSquare
        (:Valid
          (if (not false)
            (Default|SetDragState (CallFunction|GetMovingUnit) false :!label _label)
            (Variables|/Game/Test/Blueprint/Level/BP_Test_Square.BP_Test_Square_C|SetHostedUnit (Variables|Default|GetInitialMovingSquare) (CallFunction|GetMovingUnit))
            (CallFunction|InvalidMove)))
        (:Invalid
          (Default|SetDragState (CallFunction|GetMovingUnit) false)
          (Variables|/Game/Test/Blueprint/Level/BP_Test_Square.BP_Test_Square_C|SetHostedUnit (Variables|Default|GetLastFocusedSquare) (CallFunction|GetMovingUnit))
          (CallFunction|FinalStopMove))))
    (:Is%20Not%20Valid
      (Development|PrintString "Hello")
      (goto _label))))

(fn UpdateDraggedUnitLocation
  (bind _returnvalue (CallFunction|GetMovingUnit))
  (bind _returnvalue_2 (CallFunction|GetFocusedSquare))
  (bind _returnvalue_3 (Transformation|GetActorLocation _returnvalue))
  (Utilities|IsValid _returnvalue_2
    (:Is%20Valid
      (LocalVariables|SetsquareTempLoc (Transformation|GetActorLocation _returnvalue_2)))
    (:Is%20Not%20Valid
      (LocalVariables|SetsquareTempLoc (Variables|Default|GetFingerLocation))))
  (if (Variables|Default|GetbDragging)
    (Transformation|SetActorLocation _returnvalue (Math|Interpolation|VInterpTo _returnvalue_3 (Math|Vector|MakeVector (.X (Math|Vector|BreakVector (select (Variables|Default|GetbSnapMove) (LocalVariables|GetsquareTempLoc) (Variables|Default|GetFingerLocation)))) (.Y (Math|Vector|BreakVector (select (Variables|Default|GetbSnapMove) (LocalVariables|GetsquareTempLoc) (Variables|Default|GetFingerLocation)))) (.Z (Math|Vector|BreakVector _returnvalue_3))) (Variables|Default|GetDragTriggerDelay) (Variables|Default|GetMoveSpeed)) false false)))

(fn StartHolding
  (Variables|Default|SetbHolding true))

(fn StopHolding
  (CallFunction|StopDragging)
  (Variables|Default|SetbHolding false))

(fn GetUnitinSquare
  (return (Variables|/Game/Test/Blueprint/Level/BP_Test_Square.BP_Test_Square_C|GetHostedUnit (CallFunction|GetFocusedSquare))))

(fn GetMovingUnit
  (return (Variables|Default|GetMovingUnit)))