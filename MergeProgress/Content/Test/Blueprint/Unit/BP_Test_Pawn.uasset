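; Test pawn that acts as a draggable unit hosted on BP_Test_Square tiles.
; On construction and BeginPlay, FindSquare clears the previous square's HostedUnit, sphere-traces at its location, then registers with and snaps above any square hit.
; SetDragState lifts the Box component high while dragged and lowers it on release, without moving the actor.
; SetFocused is only a debug print stub.
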(event EventBeginPlay
  (CallFunction|FindSquare))

(event Collision|EventActorBeginOverlap
  (params (OtherActor :type Actor%20Object%20Reference)))

(event EventTick
  (params (DeltaSeconds :type Float%20%28single-precision%29)))

(fn ConstructionScript
  (CallFunction|FindSquare))

(fn SetFocused
  (params (bFocused :type Boolean))
  (if bFocused
    (Development|PrintString "Hello")))

(fn SetDragState
  (params (Enabled :type Boolean))
  (CallFunction|SetMeshRelativeZState Enabled))

(fn SetMeshRelativeZState
  (params (bDragged :type Boolean))
  (if bDragged
    (Transformation|SetRelativeLocation (Variables|Default|GetBox) (Math|Vector|MakeVector 0.0 0.0 2e+03) false false)
    (else
      (Transformation|SetRelativeLocation (Variables|Default|GetBox) (Math|Vector|MakeVector 0.0 0.0 -5e+01) false false))))

(fn FindSquare
  (bind _returnvalue (Transformation|GetActorLocation))
  (Variables|/Game/Test/Blueprint/Level/BP_Test_Square.BP_Test_Square_C|SetHostedUnit (Variables|Default|GetInitialSquare) 0)
  (bind _outhits (Collision|MultiSphereTraceByChannel _returnvalue (+ _returnvalue "0, 0,1.000000") 5.0 "TraceTypeQuery4" false 0 "None"))
  (for _array_element _outhits
    (if (== (Utilities|GetClass (.HitActor (Collision|BreakHitResult _array_element))) "/Game/Test/Blueprint/Level/BP_Test_Square.BP_Test_Square_C")
      (bind _asbp_test_square (Utilities|Casting|CastToBP_Test_Square (.HitActor (Collision|BreakHitResult _array_element))))
      (Variables|/Game/Test/Blueprint/Level/BP_Test_Square.BP_Test_Square_C|SetHostedUnit _asbp_test_square self)
      (Transformation|SetActorLocation (+ (Transformation|GetActorLocation _asbp_test_square) "0, 0,50.000000") false false)
      (Variables|Default|SetInitialSquare _asbp_test_square))))