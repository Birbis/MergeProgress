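; Pillar actor that spawns a neutral unit at its location.
; On BeginPlay, it fills an unset NeutroAsset from NeutriList using its index.
; Spawn_Neutro checks HostedUnit and whether the player controller's InitialMovingSquare is a BP_Square, then spawns a BP_Pawn, passing it the asset as Info and flagging it as neutral.
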(event Custom|Spawn_Neutro
  (if (== (Variables|Default|GetHostedUnit) 0)
    (bind _asbp_player_controller (Utilities|Casting|CastToBP_PlayerController (Game|GetPlayerController 0)))
    (if (== (Utilities|GetClass (Variables|/Game/MergeProgress/Player/BP_PlayerController.BP_PlayerController_C|GetInitialMovingSquare _asbp_player_controller)) "/Game/MergeProgress/Level/BP_Square.BP_Square_C")
      (bind _returnvalue (Game|SpawnActorfromClass "/Game/MergeProgress/Mergeable_Object/BP_Pawn.BP_Pawn_C" (Math|Transform|MakeTransform (Transformation|GetActorLocation self) "0,90.000000, 0") "AlwaysSpawn" 0 0 "NewEnumerator2" 0 0 0.0 0))
      (Variables|/Game/MergeProgress/Mergeable_Object/BP_Pawn.BP_Pawn_C|SetInfo _returnvalue (Variables|Default|GetNeutroAsset))
      (Variables|/Game/MergeProgress/Mergeable_Object/BP_Pawn.BP_Pawn_C|SetIsNeutro _returnvalue true))))

(event EventBeginPlay
  (if (Utilities|Name|Equal(Name) (Variables|/Game/MergeProgress/DataAssets/Animals_DataAssets/BP_ElementInfo.BP_ElementInfo_C|GetID (Variables|Default|GetNeutroAsset)) "None")
    (Variables|Default|SetNeutroAsset (Utilities|Array|Get(acopy) (Variables|Default|GetNeutriList) (Variables|Default|GetIndx)))))

(fn ConstructionScript
  (|CallParentFunction))