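; BP_SquareAPK is a level square that keeps references to its neighbouring squares (Vicini).
; On BeginPlay it caches the current level name, which SetVicini compares against Map_Prototype_City, though that branch is empty.
; AddArray appends the south, east and south-east neighbours to the Vicini array.
; A HostedUnit variable exists but is unused, and the construction script is empty.
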(event Custom|SetVicini
  (if (Utilities|Enum|Equal(Enum) (Variables|Default|GetLevelName) "Map_Prototype_City")
    _))

(event Custom|AddArray
  (bind _vicini (Variables|Default|GetVicini))
  (Utilities|Array|Add _vicini (Variables|Default|GetVicinoSud))
  (Utilities|Array|Add _vicini (Variables|Default|GetVicinoEst))
  (Utilities|Array|Add _vicini (Variables|Default|GetVicinoSudEst)))

(event EventBeginPlay
  (bind _returnvalue (Game|GetCurrentLevelName true))
  (Variables|Default|SetLevelName _returnvalue))

(fn ConstructionScript)