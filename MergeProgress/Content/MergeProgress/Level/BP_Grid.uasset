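; Grid actor that rebuilds the saved city at BeginPlay as a Width by Depth field of BP_Square tiles.
; BuildGridNew spawns squares with land and rotation from the GameInstance's CityContent, adds BP_Pawn buildings with saved residents and timers, then clears that array.
; On Map_Prototype_City only, PopulateGridVicini uses flat-index macros to link each square's neighbours up to two cells away, then calls AddArray on each.
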(event EventBeginPlay
  (bind _returnvalue (Game|GetCurrentLevelName true))
  (bind _output_get (Variables|Default|SetLevelName _returnvalue))
  (CallFunction|BuildGridNew)
  (Rendering|SetActorHiddenInGame false)
  (Collision|SetActorEnableCollision false)
  (if (Utilities|Enum|Equal(Enum) _output_get "Map_Prototype_City")
    (CallFunction|PopulateGridVicini)
    (for _array_element (Variables|Default|GetQuadrati)
      (Default|AddArray _array_element))))

(event Collision|EventActorBeginOverlap
  (params (OtherActor :type Actor%20Object%20Reference)))

(event EventTick
  (params (DeltaSeconds :type Float%20%28single-precision%29)))

(fn ConstructionScript)

(fn BuildGridNew
  (bind _width (Variables|Default|GetWidth))
  (bind _asmy_game_instance (Utilities|Casting|CastToMyGameInstance (Game|GetGameInstance)))
  (for _index (range 1 _width)
    (for _index_2 (range 1 (Variables|Default|GetDepth))
      (Development|PrintString (Utilities|String|ToString(Integer) (+ (* (- _index 1) _width) _index_2 -1)))
      (bind _returnvalue (Game|SpawnActorfromClass "/Game/MergeProgress/Level/BP_Square.BP_Square_C" (Math|Transform|MakeTransform (+ (Math|Vector|MakeVector (Math|Conversions|ToFloat(Integer) (* _index 100)) (Math|Conversions|ToFloat(Integer) (* _index_2 -100)) 1.0) (Transformation|GetActorLocation))) "AlwaysSpawn" 0 (.land (Utilities|Array|Get(acopy) (Variables|/Game/MergeProgress/GameInstance/SaveGameObject.SaveGameObject_C|GetCityContent (Variables|/Game/MergeProgress/GameInstance/MyGameInstance.MyGameInstance_C|GetSaveGameData _asmy_game_instance)) (+ (* (- _index 1) _width) _index_2 -1))) (.squarerotation (Utilities|Array|Get(acopy) (Variables|/Game/MergeProgress/GameInstance/SaveGameObject.SaveGameObject_C|GetCityContent (Variables|/Game/MergeProgress/GameInstance/MyGameInstance.MyGameInstance_C|GetSaveGameData _asmy_game_instance)) (+ (* (- _index 1) _width) _index_2 -1))) 0))
      (Utilities|Array|Add (Variables|Default|GetQuadrati) _returnvalue)))
  (for (_array_element _array_index) (Variables|/Game/MergeProgress/GameInstance/SaveGameObject.SaveGameObject_C|GetCityContent (Variables|/Game/MergeProgress/GameInstance/MyGameInstance.MyGameInstance_C|GetSaveGameData _asmy_game_instance))
    (if (!= (.building _array_element) 0)
      (bind _returnvalue_2 (Game|SpawnActorfromClass "/Game/MergeProgress/Mergeable_Object/BP_Pawn.BP_Pawn_C" (Math|Transform|MakeTransform (+ "0, 0,50.000000" (Transformation|GetActorLocation (Utilities|Array|Get(acopy) (Variables|Default|GetQuadrati) _array_index)))) "AlwaysSpawn" 0 (.building _array_element) (.buildingrotation _array_element) (.residents _array_element) (.maxresidents _array_element) (.remenaingtimer _array_element) 0))
      (Components|StaticMesh|SetStaticMesh (Variables|/Game/MergeProgress/Mergeable_Object/BP_Pawn.BP_Pawn_C|GetBuildingBody _returnvalue_2) (Utilities|Array|Get(acopy) (Variables|/Game/MergeProgress/DataAssets/Buildings_DataAssets/BP_BuildingInfo.BP_BuildingInfo_C|GetMesh (.building _array_element))))))
  (Utilities|Array|Clear (Variables|/Game/MergeProgress/GameInstance/SaveGameObject.SaveGameObject_C|GetCityContent (Variables|/Game/MergeProgress/GameInstance/MyGameInstance.MyGameInstance_C|GetSaveGameData _asmy_game_instance))))

(fn PopulateGridVicini
  (for (_array_element _array_index) (Variables|Default|GetQuadrati)
    (|VicinoSud _array_index _array_element
      (:then
        _)
      (:else
        _))
    (|VicinoEst _array_index _array_element
      (:then
        _)
      (:then2
        _))
    (|VicinoSudEst _array_index _array_element
      (:then2
        _)
      (:then
        _)
      (:else
        _))
    (|VicinoNord _array_index _array_element
      (:then2
        _)
      (:then
        _))
    (|VicinoOvest _array_index _array_element
      (:then2
        _)
      (:then
        _))
    (|VicinoSud+1 _array_index _array_element
      (:then
        _)
      (:else
        _))
    (|VicinoEst+1 _array_index _array_element
      (:then
        _)
      (:then2
        _)
      (:else
        _))
    (|VicinoNord+1 _array_index _array_element
      (:then2
        _)
      (:then
        _))
    (|VicinoOvest+1 _array_index _array_element
      (:then2
        _)
      (:else
        _)
      (:then
        _))
    (|VicinoNordEst _array_index _array_element
      (:then
        _)
      (:then2
        _)
      (:then3
        _))
    (|VicinoSudOvest _array_index _array_element
      (:then
        _)
      (:then2
        _)
      (:else
        _))
    (|VicinoNordOvest _array_index _array_element
      (:then
        _)
      (:then2
        _)
      (:then3
        _))
    (|VicinoSudEst+1 _array_index _array_element
      (:then2
        _)
      (:else
        _)
      (:else2
        _)
      (:then
        _))
    (|VicinoNordEst+1 _array_index _array_element
      (:then2
        _)
      (:then3
        _)
      (:then
        _)
      (:else
        _))
    (|VicinoSudOvest+1 _array_index _array_element
      (:then2
        _)
      (:then
        _)
      (:else2
        _)
      (:else
        _))
    (|VicinoNordOvest+1 _array_index _array_element
      (:then2
        _)
      (:then3
        _)
      (:then
        _)
      (:else
        _))
    (|VicinoSud+1Est _array_index _array_element
      (:then
        _)
      (:then2
        _)
      (:else
        _))
    (|VicinoSud+1Ovest _array_index _array_element
      (:then
        _)
      (:then2
        _)
      (:else
        _))
    (|VicinoNord+1Est _array_index _array_element
      (:then
        _)
      (:then2
        _)
      (:then3
        _))
    (|VicinoNord+1Ovest _array_index _array_element
      (:then
        _)
      (:then2
        _)
      (:then3
        _))
    (|VicinoSud+1Est+1 _array_index _array_element
      (:then
        _)
      (:else2
        _)
      (:then2
        _)
      (:else
        _))
    (|VicinoSud+1Ovest+1 _array_index _array_element
      (:then
        _)
      (:then2
        _)
      (:else2
        _)
      (:else
        _))
    (|VicinoNord+1Est+1 _array_index _array_element
      (:then
        _)
      (:then2
        _)
      (:then3
        _)
      (:else
        _))
    (|VicinoNord+1Ovest+1 _array_index _array_element)))