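; BP_SpawnChanger is a tappable level actor that switches which animal its linked Spawner uses.
; Each tap cycles six slots, falling back to the first when the next animal is undiscovered, then updates both preview meshes and the Spawner's index, sprite and CanAdvance flag.
; Quest progress from the player controller's HUD enables the colliders, with a separate first-tap collider that completes a tutorial quest and then disables itself.
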(event OnInputTouchEnd(Collider1)
  (params (FingerIndex :type ETouchIndex%20Enum :default "Touch1") (TouchedComponent :type Primitive%20Component%20Object%20Reference))
  (CallFunction|ChangeRenew))

(event OnInputTouchEnd(PrimoTap)
  (params (FingerIndex :type ETouchIndex%20Enum :default "Touch1") (TouchedComponent :type Primitive%20Component%20Object%20Reference))
  ;[1 1 1] First Tap
  (CallFunction|ChangeRenew)
  (Utilities|FlowControl|DoOnce false
    (:Completed
      (Utilities|FlowControl|RetriggerableDelay 0.5)
      (Collision|SetCollisionEnabled TouchedComponent "NoCollision")
      (bind _asbp_player_controller (Utilities|Casting|CastToBP_PlayerController (Game|GetPlayerController 0)))
      (Default|CompleteGenericQuest _asbp_player_controller)
      (CallFunction|CheckCollEvent))))

(event Custom|Change%20Renew
  (bind _spawner (Variables|Default|GetSpawner))
  (Audio|PlaySound2D "/Game/MergeProgress/Audio/Sfx/Switch_animale.Switch_animale" 1.0 1.0 0.0 0 0)
  (bind _asbp_player_controller (Utilities|Casting|CastToBP_PlayerController (Game|GetPlayerController 0)))
  (Class|SkinnedMeshComponent|SetSkeletalMesh (Variables|Default|GetRenewable1) (Variables|/Game/MergeProgress/DataAssets/Animals_DataAssets/BP_ElementInfo.BP_ElementInfo_C|GetMesh (select (.discovered (.Value (Utilities|Map|Find (Variables|/Game/MergeProgress/HUD/HUD_Gameplay.HUD_Gameplay_C|GetAnimalsInCity (Variables|/Game/MergeProgress/Player/BP_PlayerController.BP_PlayerController_C|GetHUDWidget _asbp_player_controller)) (Utilities|Array|Get(acopy) (Variables|Default|GetRenewList1) (Math|Integer|SelectInt (+ (Variables|Default|GetIndx) 1) 0 (< (Variables|Default|GetIndx) 5)))))) (Utilities|Array|Get(acopy) (Variables|Default|GetRenewList1) (Math|Integer|SelectInt (+ (Variables|Default|GetIndx) 1) 0 (< (Variables|Default|GetIndx) 5))) "/Game/MergeProgress/DataAssets/Animals_DataAssets/DA_Dog.DA_Dog")) true)
  (Class|SkinnedMeshComponent|SetSkeletalMesh (Variables|Default|GetRenewable2) (select (.discovered (.Value (Utilities|Map|Find (Variables|/Game/MergeProgress/HUD/HUD_Gameplay.HUD_Gameplay_C|GetAnimalsInCity (Variables|/Game/MergeProgress/Player/BP_PlayerController.BP_PlayerController_C|GetHUDWidget _asbp_player_controller)) (Utilities|Array|Get(acopy) (Variables|Default|GetRenewList2) (Math|Integer|SelectInt (Math|Integer|SelectInt (+ (Variables|Default|GetIndx) 1) 0 (< (Variables|Default|GetIndx) 5)) 0 (.discovered (.Value (Utilities|Map|Find (Variables|/Game/MergeProgress/HUD/HUD_Gameplay.HUD_Gameplay_C|GetAnimalsInCity (Variables|/Game/MergeProgress/Player/BP_PlayerController.BP_PlayerController_C|GetHUDWidget _asbp_player_controller)) (Utilities|Array|Get(acopy) (Variables|Default|GetRenewList1) (Math|Integer|SelectInt (+ (Variables|Default|GetIndx) 1) 0 (< (Variables|Default|GetIndx) 5))))))))))) (Variables|/Game/MergeProgress/DataAssets/Animals_DataAssets/BP_ElementInfo.BP_ElementInfo_C|GetMesh (Utilities|Array|Get(acopy) (Variables|Default|GetRenewList2) (Math|Integer|SelectInt (Math|Integer|SelectInt (+ (Variables|Default|GetIndx) 1) 0 (< (Variables|Default|GetIndx) 5)) 0 (.discovered (.Value (Utilities|Map|Find (Variables|/Game/MergeProgress/HUD/HUD_Gameplay.HUD_Gameplay_C|GetAnimalsInCity (Variables|/Game/MergeProgress/Player/BP_PlayerController.BP_PlayerController_C|GetHUDWidget _asbp_player_controller)) (Utilities|Array|Get(acopy) (Variables|Default|GetRenewList1) (Math|Integer|SelectInt (+ (Variables|Default|GetIndx) 1) 0 (< (Variables|Default|GetIndx) 5))))))))) 0) false)
  (Variables|/Game/MergeProgress/Spawner/BP_Test_AppleSpawner.BP_Test_AppleSpawner_C|SetCanAdvance _spawner (.discovered (.Value (Utilities|Map|Find (Variables|/Game/MergeProgress/HUD/HUD_Gameplay.HUD_Gameplay_C|GetAnimalsInCity (Variables|/Game/MergeProgress/Player/BP_PlayerController.BP_PlayerController_C|GetHUDWidget _asbp_player_controller)) (Utilities|Array|Get(acopy) (Variables|Default|GetRenewList2) (Math|Integer|SelectInt (Math|Integer|SelectInt (+ (Variables|Default|GetIndx) 1) 0 (< (Variables|Default|GetIndx) 5)) 0 (.discovered (.Value (Utilities|Map|Find (Variables|/Game/MergeProgress/HUD/HUD_Gameplay.HUD_Gameplay_C|GetAnimalsInCity (Variables|/Game/MergeProgress/Player/BP_PlayerController.BP_PlayerController_C|GetHUDWidget _asbp_player_controller)) (Utilities|Array|Get(acopy) (Variables|Default|GetRenewList1) (Math|Integer|SelectInt (+ (Variables|Default|GetIndx) 1) 0 (< (Variables|Default|GetIndx) 5))))))))))))
  (bind _output_get (Variables|Default|SetIndx (Math|Integer|SelectInt (Math|Integer|SelectInt (+ (Variables|Default|GetIndx) 1) 0 (< (Variables|Default|GetIndx) 5)) 0 (.discovered (.Value (Utilities|Map|Find (Variables|/Game/MergeProgress/HUD/HUD_Gameplay.HUD_Gameplay_C|GetAnimalsInCity (Variables|/Game/MergeProgress/Player/BP_PlayerController.BP_PlayerController_C|GetHUDWidget _asbp_player_controller)) (Utilities|Array|Get(acopy) (Variables|Default|GetRenewList1) (Math|Integer|SelectInt (+ (Variables|Default|GetIndx) 1) 0 (< (Variables|Default|GetIndx) 5)))))))))
  (bind _output_get_2 (Variables|/Game/MergeProgress/Spawner/BP_Test_AppleSpawner.BP_Test_AppleSpawner_C|SetIndx _spawner _output_get))
  (Default|RefreshSprite _spawner _output_get_2))

(event Custom|CheckCollEvent
  (bind _asbp_player_controller (Utilities|Casting|CastToBP_PlayerController (Game|GetPlayerController 0)))
  (bind _can_unbind (CallFunction|CheckPrimoTap _asbp_player_controller))
  (if _can_unbind
    (EventDispatchers|UnbindEventfromUpdateWorldPostQuest _asbp_player_controller (delegate Custom|CheckCollEvent))))

(event Custom|CanBeTapped
  (Variables|Default|SetCanTap (not (Variables|Default|GetCanTap))))

(event EventBeginPlay
  (bind _renewlist2 (Variables|Default|GetRenewList2))
  (bind _output (Utilities|Array|Get(acopy) _renewlist2))
  (Utilities|FlowControl|Delay 0.5)
  (bind _asbp_player_controller (Utilities|Casting|CastToBP_PlayerController (Game|GetPlayerController 0)))
  (EventDispatchers|BindEventtoChangeHUDState (Variables|/Game/MergeProgress/Player/BP_PlayerController.BP_PlayerController_C|GetHUDWidget _asbp_player_controller) (delegate Custom|CanBeTapped))
  (bind _can_unbind (CallFunction|CheckPrimoTap _asbp_player_controller))
  (if (not _can_unbind)
    (EventDispatchers|BindEventtoUpdateWorldPostQuest _asbp_player_controller (delegate Custom|CheckCollEvent))
    (Class|SkinnedMeshComponent|SetSkeletalMesh (Variables|Default|GetRenewable2) (select (.discovered (.Value (Utilities|Map|Find (Variables|/Game/MergeProgress/HUD/HUD_Gameplay.HUD_Gameplay_C|GetAnimalsInCity (Variables|/Game/MergeProgress/Player/BP_PlayerController.BP_PlayerController_C|GetHUDWidget _asbp_player_controller)) _output))) (Variables|/Game/MergeProgress/DataAssets/Animals_DataAssets/BP_ElementInfo.BP_ElementInfo_C|GetMesh _output) 0) false)
    (Variables|/Game/MergeProgress/Spawner/BP_Test_AppleSpawner.BP_Test_AppleSpawner_C|SetCanAdvance (Variables|Default|GetSpawner) (.discovered (.Value (Utilities|Map|Find (Variables|/Game/MergeProgress/HUD/HUD_Gameplay.HUD_Gameplay_C|GetAnimalsInCity (Variables|/Game/MergeProgress/Player/BP_PlayerController.BP_PlayerController_C|GetHUDWidget _asbp_player_controller)) _output))))))

(event Collision|EventActorBeginOverlap
  (params (OtherActor :type Actor%20Object%20Reference)))

(event EventTick
  (params (DeltaSeconds :type Float%20%28single-precision%29)))

(fn ConstructionScript)

(fn CheckPrimoTap
  (params (GM :type BP%20Player%20Controller%20Object%20Reference))
  (bind _hudwidget (Variables|/Game/MergeProgress/Player/BP_PlayerController.BP_PlayerController_C|GetHUDWidget GM))
  (bind _max_quest_completed (Variables|/Game/MergeProgress/HUD/HUD_Gameplay.HUD_Gameplay_C|GetMax%20Quest%20Completed _hudwidget))
  (if (>= _max_quest_completed 2)
    (Collision|SetCollisionEnabled (Variables|Default|GetCollider1) "QueryOnly")
    (if (!= _max_quest_completed 2)
      (Collision|SetCollisionEnabled (Variables|Default|GetPrimoTap) "NoCollision")
      (return true)
      (else
        (Collision|SetCollisionEnabled (Variables|Default|GetPrimoTap) "QueryOnly")))
    (else
      (Collision|SetCollisionEnabled (Variables|Default|GetCollider1) "NoCollision")
      (Collision|SetCollisionEnabled (Variables|Default|GetPrimoTap) "NoCollision")))
  (return false))

(fn CheckCanInteract
  (bind _asbp_player_controller (Utilities|Casting|CastToBP_PlayerController (Game|GetPlayerController 0)))
  (if (>= (Variables|/Game/MergeProgress/HUD/HUD_Gameplay.HUD_Gameplay_C|GetMax%20Quest%20Completed (Variables|/Game/MergeProgress/Player/BP_PlayerController.BP_PlayerController_C|GetHUDWidget _asbp_player_controller)) 9)
    (Components|DestroyComponent (Variables|Default|GetPrimoTap) :!label _label)
    (else
      (Components|DestroyComponent (Variables|Default|GetCollider1))
      (if (not (<= (Variables|/Game/MergeProgress/HUD/HUD_Gameplay.HUD_Gameplay_C|GetMax%20Quest%20Completed (Variables|/Game/MergeProgress/Player/BP_PlayerController.BP_PlayerController_C|GetHUDWidget _asbp_player_controller)) 8))
        (goto _label)))))