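; BP_Element is an actor that can be dragged across the world by touching its static mesh.
; Touch begin and end on the mesh open and close a gate on Tick.
; While open, Tick projects the first player's mouse position onto the Z=0 plane by ray-plane math and moves the actor there, held at DragHeight, without sweeping.
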(event OnInputTouchBegin(StaticMesh)
  (params (FingerIndex :type ETouchIndex%20Enum :default "Touch1") (TouchedComponent :type Primitive%20Component%20Object%20Reference))
  (bind _returnvalue (Game|GetPlayerController 0))
  (bind (_worldlocation _worlddirection) (Game|Player|ConvertMouseLocationToWorldSpace _returnvalue))
  (bind _z (Math|Vector|BreakVector _worlddirection))
  (bind _z_2 (Math|Vector|BreakVector _worldlocation))
  (bind _returnvalue_2 (/ _z_2 _z))
  (bind _returnvalue_3 (* _worlddirection _returnvalue_2))
  (bind _returnvalue_4 (* _returnvalue_3 -1.0))
  (bind _returnvalue_5 (+ _worldlocation _returnvalue_4))
  (Utilities|FlowControl|Gate true) ; enters at Open
)

(event OnInputTouchEnd(StaticMesh)
  (params (FingerIndex :type ETouchIndex%20Enum :default "Touch1") (TouchedComponent :type Primitive%20Component%20Object%20Reference))
  (bind _returnvalue (Game|GetPlayerController 0))
  (bind (_worldlocation _worlddirection) (Game|Player|ConvertMouseLocationToWorldSpace _returnvalue))
  (bind _z (Math|Vector|BreakVector _worlddirection))
  (bind _z_2 (Math|Vector|BreakVector _worldlocation))
  (bind _returnvalue_2 (/ _z_2 _z))
  (bind _returnvalue_3 (* _worlddirection _returnvalue_2))
  (bind _returnvalue_4 (* _returnvalue_3 -1.0))
  (bind _returnvalue_5 (+ _worldlocation _returnvalue_4))
  (Utilities|FlowControl|Gate true) ; enters at Close
)

(event Collision|EventActorBeginOverlap
  (params (OtherActor :type Actor%20Object%20Reference)))

(event EventTick
  (params (DeltaSeconds :type Float%20%28single-precision%29))
  (bind _returnvalue (Game|GetPlayerController 0))
  (bind (_worldlocation _worlddirection) (Game|Player|ConvertMouseLocationToWorldSpace _returnvalue))
  (bind _z (Math|Vector|BreakVector _worlddirection))
  (bind _z_2 (Math|Vector|BreakVector _worldlocation))
  (bind _returnvalue_2 (/ _z_2 _z))
  (bind _returnvalue_3 (* _worlddirection _returnvalue_2))
  (bind _returnvalue_4 (* _returnvalue_3 -1.0))
  (bind _returnvalue_5 (+ _worldlocation _returnvalue_4))
  (Utilities|FlowControl|Gate true
    (:Exit
      (Transformation|SetActorLocation (Math|Vector|MakeVector (.x _returnvalue_5) (.y _returnvalue_5) (Variables|Default|GetDragHeight)) false false))))

(fn ConstructionScript)