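; BP_Pawn is a grid unit that serves as either an animal or a building in a merge and city-building game.
; Birth and Buildthebuilding dress it as one or the other, with timed construction that updates HUD building counts, capacity or income.
; FindSquare sphere-traces to claim its BP_Square, snapping and filling neighbor squares by footprint in the city.
; It also handles drag state, touch-opened building HUD and moving animals into saved boat slots.
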(event Custom|Birth
  (bind _info (Variables|Default|GetInfo))
  (bind _animalbody (Variables|Default|GetAnimalBody))
  (bind _info_2 (Variables|Default|GetInfo))
  ;[1 1 1] Al momento dello spawn dell'animale setta mesh, materiale e animazioni
  (Utilities|FlowControl|Sequence
    (:then_0
      (Class|SkinnedMeshComponent|SetSkeletalMesh _animalbody (Variables|/Game/MergeProgress/DataAssets/Animals_DataAssets/BP_ElementInfo.BP_ElementInfo_C|GetMesh _info) true)
      (Rendering|Material|SetMaterial _animalbody 0 (Variables|/Game/MergeProgress/DataAssets/Animals_DataAssets/BP_ElementInfo.BP_ElementInfo_C|GetMaterial _info))
      (Development|SetHiddeninGame (Variables|Default|GetBuildingBody) true false))
    (:then_1
      (Variables|Default|SetSpawned true)
      (Utilities|FlowControl|Delay 1.0)
      (Variables|Default|SetSpawned false)
      (bind _asbp_player_controller (Utilities|Casting|CastToBP_PlayerController (Game|GetPlayerController 0)))
      (Utilities|Map|Add (Variables|/Game/MergeProgress/HUD/HUD_Gameplay.HUD_Gameplay_C|GetAnimalsInCity (Variables|/Game/MergeProgress/Player/BP_PlayerController.BP_PlayerController_C|GetHUDWidget _asbp_player_controller)) _info_2 (Utilities|Struct|MakeDS_AnimalInfo (.discovered (.Value (Utilities|Map|Find (Variables|/Game/MergeProgress/HUD/HUD_Gameplay.HUD_Gameplay_C|GetAnimalsInCity (Variables|/Game/MergeProgress/Player/BP_PlayerController.BP_PlayerController_C|GetHUDWidget _asbp_player_controller)) _info_2))) (.qjobless (.Value (Utilities|Map|Find (Variables|/Game/MergeProgress/HUD/HUD_Gameplay.HUD_Gameplay_C|GetAnimalsInCity (Variables|/Game/MergeProgress/Player/BP_PlayerController.BP_PlayerController_C|GetHUDWidget _asbp_player_controller)) _info_2))) (.qworking (.Value (Utilities|Map|Find (Variables|/Game/MergeProgress/HUD/HUD_Gameplay.HUD_Gameplay_C|GetAnimalsInCity (Variables|/Game/MergeProgress/Player/BP_PlayerController.BP_PlayerController_C|GetHUDWidget _asbp_player_controller)) _info_2))) (.qworkerbytype (.Value (Utilities|Map|Find (Variables|/Game/MergeProgress/HUD/HUD_Gameplay.HUD_Gameplay_C|GetAnimalsInCity (Variables|/Game/MergeProgress/Player/BP_PlayerController.BP_PlayerController_C|GetHUDWidget _asbp_player_controller)) _info_2))) false 0.0 false)))))

(event Custom|Build%20the%20building
  (bind _remenaingtimer (Variables|Default|GetRemenaingTimer))
  (bind _returnvalue (!= _remenaingtimer 0.0))
  ;[1 1 1] Settaggio dei valori giusti allo spawning dell'edificio
  (if _returnvalue
    (if (> _remenaingtimer 0.9)
      (bind _asbp_player_controller (Utilities|Casting|CastToBP_PlayerController (Game|GetPlayerController 0)))
      (Variables|/Game/MergeProgress/HUD/HUD_Gameplay.HUD_Gameplay_C|SetIsConstructing (Variables|/Game/MergeProgress/Player/BP_PlayerController.BP_PlayerController_C|GetHUDWidget _asbp_player_controller) true)
      (CallFunction|StartConstructing)
      (Components|StaticMesh|SetStaticMesh (Variables|Default|GetBuildingBody) (select _returnvalue (Variables|Default|GetConstructionMesh) (Utilities|Array|Get(acopy) (Variables|/Game/MergeProgress/DataAssets/Buildings_DataAssets/BP_BuildingInfo.BP_BuildingInfo_C|GetMesh (Variables|Default|GetInfo_Building)) (Variables|Default|GetLivello))) :!label _label)
      (Development|SetHiddeninGame (Variables|Default|GetAnimalBody) true false)
      (Transformation|SetRelativeRotation (Variables|Default|GetBuildingBody) (Utilities|Select :Index (Variables|Default|GetCardinal) :NewEnumerator0 "0,180.000000, 0" :NewEnumerator1 "0,270.000000, 0" :NewEnumerator2 "0, 0, 0" :NewEnumerator3 "0,90.000000, 0") false false)
      (else
        (CallFunction|FinishConstructing)))
    (else
      (goto _label))))

(event Custom|Finish%20Constructing
  (bind _info_building (Variables|Default|GetInfo_Building))
  ;[1 1 1] Logica Costruzione
  (Variables|Default|SetRemenaingTimer 0.0)
  (bind _asbp_player_controller (Utilities|Casting|CastToBP_PlayerController (Game|GetPlayerController 0)))
  (Variables|/Game/MergeProgress/HUD/HUD_Gameplay.HUD_Gameplay_C|SetIsConstructing (Variables|/Game/MergeProgress/Player/BP_PlayerController.BP_PlayerController_C|GetHUDWidget _asbp_player_controller) false)
  (Components|StaticMesh|SetStaticMesh (Variables|Default|GetBuildingBody) (Utilities|Array|Get(acopy) (Variables|/Game/MergeProgress/DataAssets/Buildings_DataAssets/BP_BuildingInfo.BP_BuildingInfo_C|GetMesh (Variables|Default|GetInfo_Building)) (Variables|Default|GetLivello)))
  (Utilities|Time|ClearandInvalidateTimerbyHandle (Variables|Default|GetConstructTimerHandler))
  (Utilities|Map|Add (Variables|/Game/MergeProgress/HUD/HUD_Gameplay.HUD_Gameplay_C|GetBuildings (Variables|/Game/MergeProgress/Player/BP_PlayerController.BP_PlayerController_C|GetHUDWidget _asbp_player_controller)) _info_building (Utilities|Struct|MakeDS_BuildingInfo (.discovered (.Value (Utilities|Map|Find (Variables|/Game/MergeProgress/HUD/HUD_Gameplay.HUD_Gameplay_C|GetBuildings (Variables|/Game/MergeProgress/Player/BP_PlayerController.BP_PlayerController_C|GetHUDWidget _asbp_player_controller)) _info_building))) (+ (.howmany (.Value (Utilities|Map|Find (Variables|/Game/MergeProgress/HUD/HUD_Gameplay.HUD_Gameplay_C|GetBuildings (Variables|/Game/MergeProgress/Player/BP_PlayerController.BP_PlayerController_C|GetHUDWidget _asbp_player_controller)) _info_building))) 1) (.feature (.Value (Utilities|Map|Find (Variables|/Game/MergeProgress/HUD/HUD_Gameplay.HUD_Gameplay_C|GetBuildings (Variables|/Game/MergeProgress/Player/BP_PlayerController.BP_PlayerController_C|GetHUDWidget _asbp_player_controller)) _info_building))) true (.level (.Value (Utilities|Map|Find (Variables|/Game/MergeProgress/HUD/HUD_Gameplay.HUD_Gameplay_C|GetBuildings (Variables|/Game/MergeProgress/Player/BP_PlayerController.BP_PlayerController_C|GetHUDWidget _asbp_player_controller)) _info_building))) (.residents (.Value (Utilities|Map|Find (Variables|/Game/MergeProgress/HUD/HUD_Gameplay.HUD_Gameplay_C|GetBuildings (Variables|/Game/MergeProgress/Player/BP_PlayerController.BP_PlayerController_C|GetHUDWidget _asbp_player_controller)) _info_building))) (.maxresidents (.Value (Utilities|Map|Find (Variables|/Game/MergeProgress/HUD/HUD_Gameplay.HUD_Gameplay_C|GetBuildings (Variables|/Game/MergeProgress/Player/BP_PlayerController.BP_PlayerController_C|GetHUDWidget _asbp_player_controller)) _info_building))) (.moneygainbuilding (.Value (Utilities|Map|Find (Variables|/Game/MergeProgress/HUD/HUD_Gameplay.HUD_Gameplay_C|GetBuildings (Variables|/Game/MergeProgress/Player/BP_PlayerController.BP_PlayerController_C|GetHUDWidget _asbp_player_controller)) _info_building)))))
  (bind _output_get (Variables|Default|SetPawnType (Variables|/Game/MergeProgress/DataAssets/Buildings_DataAssets/BP_BuildingInfo.BP_BuildingInfo_C|GetBuildingType _info_building)))
  (switch Utilities|FlowControl|Switch|SwitchonEBuildingFeature _output_get
    (:NewEnumerator4
      (Variables|/Game/MergeProgress/HUD/HUD_Gameplay.HUD_Gameplay_C|SetAnimals%20Max%20Capacity (Variables|/Game/MergeProgress/Player/BP_PlayerController.BP_PlayerController_C|GetHUDWidget _asbp_player_controller) (+ (.maxresidents (.Value (Utilities|Map|Find (Variables|/Game/MergeProgress/HUD/HUD_Gameplay.HUD_Gameplay_C|GetBuildings (Variables|/Game/MergeProgress/Player/BP_PlayerController.BP_PlayerController_C|GetHUDWidget _asbp_player_controller)) _info_building))) (Variables|/Game/MergeProgress/HUD/HUD_Gameplay.HUD_Gameplay_C|GetAnimals%20Max%20Capacity (Variables|/Game/MergeProgress/Player/BP_PlayerController.BP_PlayerController_C|GetHUDWidget _asbp_player_controller)))))
    (:NewEnumerator7
      (Variables|/Game/MergeProgress/HUD/HUD_Gameplay.HUD_Gameplay_C|SetMoneyGain (Variables|/Game/MergeProgress/Player/BP_PlayerController.BP_PlayerController_C|GetHUDWidget _asbp_player_controller) (+ (Variables|/Game/MergeProgress/HUD/HUD_Gameplay.HUD_Gameplay_C|GetMoneyGain (Variables|/Game/MergeProgress/Player/BP_PlayerController.BP_PlayerController_C|GetHUDWidget _asbp_player_controller)) (.moneygainbuilding (.Value (Utilities|Map|Find (Variables|/Game/MergeProgress/HUD/HUD_Gameplay.HUD_Gameplay_C|GetBuildings (Variables|/Game/MergeProgress/Player/BP_PlayerController.BP_PlayerController_C|GetHUDWidget _asbp_player_controller)) _info_building)))) :!label _label))
    (:NewEnumerator6
      (goto _label))
    (:NewEnumerator1
      (goto _label))
    (:NewEnumerator2
      (goto _label))
    (:NewEnumerator8
      (goto _label))
    (:NewEnumerator3
      (goto _label))
    (:NewEnumerator5
      (goto _label))))

(event Custom|StartConstructing
  ;[1 1 1] Logica Costruzione
  (bind _returnvalue (Utilities|Time|SetTimerbyEvent (delegate Custom|Finish%20Constructing) (Variables|Default|GetRemenaingTimer) false 0.1))
  (Variables|Default|SetConstructTimerHandler _returnvalue))

(event Custom|UpgradeLevelBuilding
  (Math|Integer|IncrementInt (Variables|Default|GetLivello)
    (:%20%20
      (CallFunction|BuildtheBuilding))))

(event Custom|CustomEvent_0)

(event EventBeginPlay
  ;[0 1 0.2468] BeginPlay
  (bind _returnvalue (Game|GetCurrentLevelName true))
  (Variables|Default|SetLevelName _returnvalue)
  (Utilities|FlowControl|Delay 0.05)
  (CallFunction|FindSquare))

(event EventActorOnInputTouchBegin
  (params (FingerIndex :type ETouchIndex%20Enum :default "Touch1"))
  (bind _asbp_player_controller (Utilities|Casting|CastToBP_PlayerController (Game|GetPlayerController 0)))
  (if (not (or (Variables|/Game/MergeProgress/Player/BP_PlayerController.BP_PlayerController_C|GetHUDOn _asbp_player_controller) (Variables|/Game/MergeProgress/Player/BP_PlayerController.BP_PlayerController_C|GetIsBuild _asbp_player_controller)))
    (Default|ShowBuildingHud (Variables|/Game/MergeProgress/Player/BP_PlayerController.BP_PlayerController_C|GetHUDWidget _asbp_player_controller) self)))

(fn ConstructionScript)

(fn SetFocused
  (params (bFocused :type Boolean)))

(fn SetDragState
  (params (Enabled :type Boolean))
  (CallFunction|SetMeshRelativeZState Enabled)
  (Variables|Default|SetDragged Enabled)
  (if (!= (Variables|Default|GetInfo_Building) 0)
    (Collision|SetCollisionProfileName (Variables|Default|GetBuildingBody) (select Enabled "NoCollision" "Pawn") true :!class /Script/Engine.PrimitiveComponent)))

(fn SetMeshRelativeZState
  (params (bDragged :type Boolean))
  (bind _returnvalue (Transformation|GetActorLocation))
  (if bDragged
    (Transformation|SetRelativeLocation (Variables|Default|GetBox) (Math|Vector|MakeVector (.x _returnvalue) (.y _returnvalue) (select (Utilities|Enum|Equal(Enum) (Variables|Default|GetLevelName) "Map_Prototype_City") (Variables|Default|GetAltezzaBuilding) (LocalVariables|GetAltezza))) false false)
    (else
      (Transformation|SetRelativeLocation (Variables|Default|GetBox) (Math|Vector|MakeVector (.x _returnvalue) (.y _returnvalue) 1e+02) false false))))

(fn FindSquare
  (bind _returnvalue (Transformation|GetActorLocation))
  (if (== (Variables|Default|GetInfo_Building) 0)
    _
    (else
      _))
  (bind _outhits (Collision|MultiSphereTraceByChannel _returnvalue (+ _returnvalue "0, 0,1.000000") 1.0 "TraceTypeQuery4" false 0 "None"))
  (for _array_element _outhits
    (bind _asbp_square (Utilities|Casting|CastToBP_Square (.HitActor (Collision|BreakHitResult _array_element))))
    (bind _asbp_player_controller (Utilities|Casting|CastToBP_PlayerController (Game|GetPlayerController 0)))
    (if (Utilities|Name|Equal(Name) (Variables|/Game/MergeProgress/Player/BP_PlayerController.BP_PlayerController_C|GetCurrentLevelName _asbp_player_controller) (Variables|/Game/MergeProgress/Player/BP_PlayerController.BP_PlayerController_C|GetCityLevelName _asbp_player_controller))
      (Variables|/Game/MergeProgress/Level/BP_Square.BP_Square_C|SetHostedUnit _asbp_square self)
      (Transformation|SetActorLocation (+ (Transformation|GetActorLocation _asbp_square) (Variables|/Game/MergeProgress/DataAssets/Buildings_DataAssets/BP_BuildingInfo.BP_BuildingInfo_C|GetAllineamento (Variables|Default|GetInfo_Building))) false false)
      (bind _output_get (Variables|Default|SetInitialSquare _asbp_square))
      (CallFunction|SetHostedUnitVicini _output_get)
      (else
        (Variables|/Game/MergeProgress/Level/BP_Square.BP_Square_C|SetHostedUnit _asbp_square self)
        (Transformation|SetActorLocation (+ (Transformation|GetActorLocation) "0.000000,0.000000,10.000000") false false)
        (Variables|Default|SetInitialSquare _asbp_square)))))

(fn AddtoBoat
  (bind _asmy_game_instance (Utilities|Casting|CastToMyGameInstance (Game|GetGameInstance)))
  (if (<= (Variables|/Game/MergeProgress/GameInstance/SaveGameObject.SaveGameObject_C|GetNumberAnimalsBoat (Variables|/Game/MergeProgress/GameInstance/MyGameInstance.MyGameInstance_C|GetSaveGameData _asmy_game_instance)) 11)
    (Math|Integer|IncrementInt (Variables|/Game/MergeProgress/GameInstance/SaveGameObject.SaveGameObject_C|GetNumberAnimalsBoat (Variables|/Game/MergeProgress/GameInstance/MyGameInstance.MyGameInstance_C|GetSaveGameData _asmy_game_instance))
      (:%20%20
        (bind _asbp_player_controller (Utilities|Casting|CastToBP_PlayerController (Game|GetPlayerController 0)))
        (bind _array_element (Utilities|Array|ForEachLoopwithBreak (Class|PanelWidget|GetAllChildren (Variables|/Game/MergeProgress/HUD/HUD_Gameplay.HUD_Gameplay_C|GetBoat_Grid (Variables|/Game/MergeProgress/Player/BP_PlayerController.BP_PlayerController_C|GetHUDWidget _asbp_player_controller))) :!label _label)
          (:LoopBody
            (bind _ashud_slot_animal (Utilities|Casting|CastToHUD_Slot_Animal _array_element))
            (if (== (Variables|/Game/MergeProgress/HUD/HUD_Slot_Animal.HUD_Slot_Animal_C|GetAnimal _ashud_slot_animal) 0)
              (bind _output_get (Variables|/Game/MergeProgress/HUD/HUD_Slot_Animal.HUD_Slot_Animal_C|SetAnimal _ashud_slot_animal (Variables|Default|GetInfo)))
              (Utilities|Array|Add (Variables|/Game/MergeProgress/GameInstance/SaveGameObject.SaveGameObject_C|GetAnimalsInBoat (Variables|/Game/MergeProgress/GameInstance/MyGameInstance.MyGameInstance_C|GetSaveGameData _asmy_game_instance)) _output_get)
              (Widget|SetVisibility (Variables|/Game/MergeProgress/HUD/HUD_Slot_Animal.HUD_Slot_Animal_C|GetIcona_Image _ashud_slot_animal) "SelfHitTestInvisible")
              (goto _label Break)))
          (:Completed
            (Actor|DestroyActor)))))))

(fn SetHostedUnitVicini
  (params (InitialSquare :type BP%20Square%20Object%20Reference))
  (for _array_element (Utilities|Select :Index (Variables|/Game/MergeProgress/DataAssets/Buildings_DataAssets/BP_BuildingInfo.BP_BuildingInfo_C|GetLarge (Variables|Default|GetInfo_Building)) :NewEnumerator0 0 :NewEnumerator1 (Variables|/Game/MergeProgress/Level/BP_Square.BP_Square_C|GetVicini_2*2 InitialSquare) :NewEnumerator2 (Variables|/Game/MergeProgress/Level/BP_Square.BP_Square_C|GetVicini_3*3 InitialSquare) :NewEnumerator3 (Variables|/Game/MergeProgress/Level/BP_Square.BP_Square_C|GetVicini_2*1 InitialSquare) :NewEnumerator4 (Variables|/Game/MergeProgress/Level/BP_Square.BP_Square_C|GetVicini_1*2 InitialSquare) :NewEnumerator5 (Variables|/Game/MergeProgress/Level/BP_Square.BP_Square_C|GetVicini_2*3 InitialSquare) :NewEnumerator6 (Variables|/Game/MergeProgress/Level/BP_Square.BP_Square_C|GetVicini_3*2 InitialSquare) :NewEnumerator7 (Variables|/Game/MergeProgress/Level/BP_Square.BP_Square_C|GetVicini_3*1 InitialSquare) :NewEnumerator8 (Variables|/Game/MergeProgress/Level/BP_Square.BP_Square_C|GetVicini_1*3 InitialSquare))
    (Variables|/Game/MergeProgress/Level/BP_Square.BP_Square_C|SetHostedUnit _array_element (Variables|/Game/MergeProgress/Level/BP_Square.BP_Square_C|GetHostedUnit InitialSquare))))

(fn SetSlotNewOrder
  ;[1 1 1] WIP
  (bind _asbp_player_controller (Utilities|Casting|CastToBP_PlayerController (Game|GetPlayerController 0)))
  (bind _array_element (Utilities|Array|ForEachLoopwithBreak (Class|PanelWidget|GetAllChildren (Variables|/Game/MergeProgress/HUD/HUD_Gameplay.HUD_Gameplay_C|GetInventoryGrid (Variables|/Game/MergeProgress/Player/BP_PlayerController.BP_PlayerController_C|GetHUDWidget _asbp_player_controller))))
    (:LoopBody
      (Utilities|Casting|CastToHUD_Slot_Animal _array_element)
      (if true
        _))))