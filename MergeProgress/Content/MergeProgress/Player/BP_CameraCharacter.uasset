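; Player camera character that handles pinch-to-zoom by changing its spring arm length.
; Pinch gestures set IsPinched on BP_PlayerController, while the PinchZoom axis compares successive values and feeds the change to PinchZooming.
; PinchZooming switches the target length between minimum and maximum distance and prints debug values; ZoomSmooth interpolates toward that target while not dragging.
; An older two-finger distance zoom remains but is disconnected.
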(event EventBeginPlay)

(event Collision|EventActorBeginOverlap
  (params (OtherActor :type Actor%20Object%20Reference)))

(event EventTick
  (params (DeltaSeconds :type Float%20%28single-precision%29)))

(event Input|AxisEvents|InputAxisPinchZoom
  (params (AxisValue :type Float%20%28single-precision%29))
  (if (not (Variables|Default|GetbDragging))
    (CallFunction|ZoomSmooth)
    (if (not (== AxisValue (Variables|Default|GetPinchValue)))
      (Math|Float|CompareFloat AxisValue (Variables|Default|GetPinchValue)
        (:>
          (CallFunction|PinchZooming (- (Math|Float|Clamp(Float) (/ (Variables|Default|GetPinchValue) AxisValue)) (Variables|Default|GetCameraZoomSpeed))))
        (:<
          (CallFunction|PinchZooming (- (Variables|Default|GetCameraZoomSpeed) (Math|Float|Clamp(Float) (/ AxisValue (Variables|Default|GetPinchValue)))))))
      (Variables|Default|SetPinchValue AxisValue))))

(event Input|TouchEvents|Touch2
  (params (Key :type Key%20Structure :default "None"))
  ;[1 1 1] Zoom logic
  (:Pressed
    (bind _distance (CallFunction|ZoomTouch))
    (Variables|Default|SetInitZoomDistance _distance)))

(event Input|KeyboardEvents|GesturePinch
  (params (Key :type Key%20Structure :default "None"))
  (:Pressed
    (bind _asbp_player_controller (Utilities|Casting|CastToBP_PlayerController (Game|GetPlayerController 0)))
    (Variables|/Game/MergeProgress/Player/BP_PlayerController.BP_PlayerController_C|SetisPinched _asbp_player_controller true)
    (Utilities|FlowControl|DoOnce false :!label _label
      (:Completed
        (Variables|Default|SetPinchValue 1.0))))
  (:Released
    (Variables|Default|SetZoommed true)
    (bind _asbp_player_controller_2 (Utilities|Casting|CastToBP_PlayerController (Game|GetPlayerController 0)))
    (Variables|/Game/MergeProgress/Player/BP_PlayerController.BP_PlayerController_C|SetisPinched _asbp_player_controller_2 false)
    (goto _label Reset)))

(event Input|TouchEvents|InputTouch
  (params (Location :type Vector) (FingerIndex :type ETouchIndex%20Enum)))

(fn ConstructionScript
  (Variables|Default|SetcameraArmLenght (Variables|/Script/Engine.SpringArmComponent|GetTargetArmLength (Variables|Default|GetSpringArm))))

(fn ZoomTouch)

(fn PinchZooming
  (params (PinchValue :type Float%20%28single-precision%29))
  (Development|PrintString (Utilities|String|ToString(Float) (Variables|Default|GetPinchValue)))
  (if (>= (Variables|Default|GetPinchValue) 1e+01)
    (Variables|Default|SetcameraArmLenght (Variables|Default|GetMinCameraDistance))
    (Variables|Default|SetZoommed false)
    (elif (<= (Variables|Default|GetPinchValue) 0.5)
      (if (Variables|Default|GetZoommed)
        (Variables|Default|SetcameraArmLenght (Variables|Default|GetMaxCameraDistance))
        (Variables|Default|SetZoommed false)))))

(fn ZoomSmooth
  (bind _springarm (Variables|Default|GetSpringArm))
  (Variables|/Script/Engine.SpringArmComponent|SetTargetArmLength _springarm (Math|Interpolation|FInterpTo (Variables|/Script/Engine.SpringArmComponent|GetTargetArmLength _springarm) (Variables|Default|GetcameraArmLenght) (Utilities|Time|GetWorldDeltaSeconds) 5.0)))