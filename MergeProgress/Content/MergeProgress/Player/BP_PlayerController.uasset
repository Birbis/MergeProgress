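; Touch player controller for a merge game, handling swipes and drag-and-drop of units between grid squares.
; Each tick it sphere-traces under the finger to focus a BP_Square, picks up its hosted unit and interpolates it toward the finger or snapped square.
; On release the unit settles on an empty square, returns to its origin, or merges by recipe into a new BP_Pawn.
; Merge results update renewable spawn counts and timers on the spawner pawn.
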(event Custom|MergeDone
  (bind _returnvalue (CallFunction|GetFocusedSquare))
  ;[1 1 1] Merge has been executed on the chosen element
  (Utilities|IsValid _returnvalue
    (:Is%20Valid
      _)
    (:Is%20Not%20Valid
      (Default|SetFocused (Variables|Default|GetMovingUnit) false)))
  (Variables|Default|SetMovingUnit 0)
  (Variables|Default|SetbDragging false)
  (Variables|Default|SetbHolding false)
  (Variables|/Game/MergeProgress/Level/BP_Square.BP_Square_C|SetHostedUnit _returnvalue 0))

(event Custom|InvalidMove
  ;[1 1 1] Invalid move, reposition object to starting point
  (Components|MoveComponentTo (Variables|/Script/Engine.Actor|GetRootComponent (Variables|Default|GetMovingUnit)) (+ (Transformation|GetActorLocation (Variables|Default|GetInitialMovingSquare)) "0, 0,30.000000") "0, 0, 0" true false (Variables|Default|GetFinalMoveDuration) false)
  (Utilities|IsValid (CallFunction|GetFocusedSquare)
    (:Is%20Valid
      _)
    (:Is%20Not%20Valid
      (Default|SetFocused (Variables|Default|GetMovingUnit) false)))
  (Variables|Default|SetMovingUnit 0)
  (Variables|Default|SetbDragging false)
  (Variables|Default|SetbHolding false))

(event Custom|FinalStopMove
  ;[1 1 1] Move element to selected square
  (Components|MoveComponentTo (Variables|/Script/Engine.Actor|GetRootComponent (Variables|Default|GetMovingUnit)) (+ (Transformation|GetActorLocation (Variables|Default|GetLastFocusedSquare)) "0, 0,30.000000") "0, 0, 0" true false (Variables|Default|GetFinalMoveDuration) false)
  (Utilities|IsValid (CallFunction|GetFocusedSquare)
    (:Is%20Valid
      _)
    (:Is%20Not%20Valid
      (Default|SetFocused (Variables|Default|GetMovingUnit) false)))
  (Variables|Default|SetMovingUnit 0)
  (Variables|Default|SetbDragging false)
  (Variables|Default|SetbHolding false))

(event Custom|DragCoords
  (params (ScreenSpace :type Vector%202D%20Structure) (ActorPayload :type Actor%20Object%20Reference))
  (bind _pixelposition (Class|SlateBlueprintLibrary|AbsolutetoViewport ScreenSpace))
  (bind _self self)
  (bind (_worldposition _worlddirection) (Class|GameplayStatics|DeprojectScreentoWorld _self _pixelposition))
  (bind _outhit (Collision|LineTraceByChannel (Transformation|GetActorLocation (Game|GetPlayerCameraManager 0)) (+ _worldposition (* _worlddirection 5e+03)) "TraceTypeQuery1" true 0 "None"))
  (Transformation|SetActorLocation ActorPayload (.Location (Collision|BreakHitResult _outhit)) false false))

(event EventTick
  (params (DeltaSeconds :type Float%20%28single-precision%29))
  (bind _returnvalue (Game|GetPlayerController 0))
  (bind (_locationx _locationy) (Class|PlayerController|GetInputTouchState _returnvalue "Touch1"))
  (bind _returnvalue_2 (Math|Vector2D|MakeVector2D _locationx _locationy))
  (|CallParentFunction DeltaSeconds)
  (CallFunction|FindFocusedSquare)
  (CallFunction|UpdateDraggedUnitLocation)
  (Utilities|FlowControl|Gate true
    (:Exit
      (if (not (Variables|Default|GetbDragging))
        (if (>= (Math|Vector2D|Vector2DLength (- _returnvalue_2 (stale Input|ActionEvents|InputActionFinger1 _output_get))) (Variables|Default|GetSwipeThreshold))
          (Variables|Default|SetStartLoc "(X=9999999980506447872.000000,Y=9999999980506447872.000000)")
          (Variables|Default|SetX (.y (* (- _returnvalue_2 (Variables|Default|GetPriorLoc)) (Variables|Default|GetSwipeSpeed))))
          (Variables|Default|SetY (.x (* (- _returnvalue_2 (Variables|Default|GetPriorLoc)) (Variables|Default|GetSwipeSpeed))))
          (Variables|Default|SetPriorLoc _returnvalue_2)
          (Variables|Default|SetSwiping true))))))

(event Input|ActionEvents|InputActionFinger1
  (params (Key :type Key%20Structure))
  (bind _returnvalue (Game|GetPlayerController 0))
  (bind (_locationx _locationy) (Class|PlayerController|GetInputTouchState _returnvalue "Touch1"))
  (bind _returnvalue_2 (Math|Vector2D|MakeVector2D _locationx _locationy))
  (:Pressed
    (bind _output_get (Variables|Default|SetStartLoc _returnvalue_2))
    (Variables|Default|SetPriorLoc _output_get)
    (Utilities|FlowControl|Gate true) ; enters at Open
  )
  (:Released
    (Variables|Default|SetSwiping false)
    (Utilities|FlowControl|Gate true) ; enters at Close
  ))

(event Input|TouchEvents|InputTouch
  (params (Location :type Vector) (FingerIndex :type ETouchIndex%20Enum))
  (:Pressed
    ;[1 1 1] Drag'N'Drop logic
    (CallFunction|UnfocusSquare)
    (Variables|Default|SetbFocusing true))
  (:Released
    (Variables|Default|SetbFocusing false)
    (if (not (not (Variables|Default|GetbDragging)))
      (if (not (Variables|Default|GetbHolding))
        (CallFunction|StopHolding)
        (Variables|Default|SetbFocusing false)
        (Variables|Default|SetPressed false)))))

(fn ConstructionScript)

(fn FindFocusedSquare
  (if (not (Variables|Default|GetSwiping))
    (if (not (Variables|Default|GetisPinched))
      (if (Variables|Default|GetbFocusing)
        (bind _output_get (Variables|Default|SetFingerLocation (.ImpactPoint (Collision|BreakHitResult (.HitResult (Class|PlayerController|GetHitResultUnderFingerbyChannel "Touch1" "TraceTypeQuery1" (.bIsCurrentlyPressed (Class|PlayerController|GetInputTouchState (Variables|Default|GetFinger%20Index_0)))))))))
        (bind _outhits (Collision|MultiSphereTraceByChannel _output_get (+ _output_get "0, 0,50.000000") 1.0 "TraceTypeQuery4" false 0 "ForOneFrame"))
        (Utilities|IsValid (.HitActor (Collision|BreakHitResult (Utilities|Array|Get(acopy) _outhits)))
          (:Is%20Valid
            (bind _asbp_square (Utilities|Casting|CastToBP_Square (.HitActor (Collision|BreakHitResult (Utilities|Array|Get(acopy) _outhits))))
              (:then
                (if (!= _asbp_square (Variables|Default|GetFocusedSquare))
                  (CallFunction|UnfocusSquare)
                  (CallFunction|SetFocusedSquare _asbp_square)
                  (else
                    (Rendering|Debug|DrawDebugPoint (Transformation|GetActorLocation _asbp_square) 1e+01 "(R=1.000000,G=0.402425,B=0.000000,A=1.000000)" 0.0))))
              (:CastFailed
                (CallFunction|UnfocusSquare :!label _label))))
          (:Is%20Not%20Valid
            (goto _label)))))))

(fn SetFocusedSquare
  (params (Square :type BP%20Square%20Object%20Reference))
  (Variables|Default|SetFocusedSquare Square)
  (if (not (Variables|Default|GetbDragging))
    (Utilities|IsThereUnitinFocusedSquare
      (:Valid
        (Default|SetFocused (CallFunction|GetUnitinSquare) true)
        (CallFunction|StartDragging)))))

(fn UnfocusSquare
  (Utilities|IsValid (CallFunction|GetFocusedSquare)
    (:Is%20Valid
      (if (not (Variables|Default|GetbDragging))
        (Utilities|IsThereUnitinFocusedSquare
          (:Valid
            (Default|SetFocused (CallFunction|GetUnitinSquare) false))
          (:Invalid
            _))))
    (:Is%20Not%20Valid
      _))
  (Utilities|IsValid (Variables|Default|GetFocusedSquare)
    (:Is%20Valid
      (Variables|Default|SetLastFocusedSquare (Variables|Default|GetFocusedSquare)))
    (:Is%20Not%20Valid
      _))
  (Variables|Default|SetFocusedSquare 0))

(fn GetFocusedSquare
  (return (Variables|Default|GetFocusedSquare)))

(fn StartDragging
  (bind _returnvalue (CallFunction|GetFocusedSquare))
  (Variables|Default|SetMovingUnit (CallFunction|GetUnitinSquare))
  (Variables|Default|SetbDragging true)
  (Default|SetDragState (CallFunction|GetMovingUnit) true)
  (Variables|Default|SetInitialMovingSquare _returnvalue)
  (Variables|/Game/MergeProgress/Level/BP_Square.BP_Square_C|SetHostedUnit _returnvalue (Variables|Default|GetHosted%20Unit)))

(fn StopDragging
  (bind _returnvalue (CallFunction|GetFocusedSquare))
  (bind _returnvalue_2 (CallFunction|GetMovingUnit))
  (bind _returnvalue_3 (CallFunction|GetUnitinSquare))
  (Utilities|IsValid _returnvalue
    (:Is%20Valid
      (Variables|Default|SetLastFocusedSquare _returnvalue)
      (Utilities|IsThereUnitinFocusedSquare
        (:Valid
          (if (Utilities|IsValid _returnvalue_3)
            (CallFunction|StartMerging _returnvalue_2 _returnvalue_3)
            (else
              (Default|SetDragState _returnvalue_2 false :!label _label)
              (Variables|/Game/MergeProgress/Level/BP_Square.BP_Square_C|SetHostedUnit (Variables|Default|GetInitialMovingSquare) _returnvalue_2)
              (CallFunction|InvalidMove))))
        (:Invalid
          (Default|SetDragState _returnvalue_2 false)
          (Variables|/Game/MergeProgress/Level/BP_Square.BP_Square_C|SetHostedUnit (Variables|Default|GetLastFocusedSquare) _returnvalue_2)
          (CallFunction|FinalStopMove))))
    (:Is%20Not%20Valid
      (goto _label))))

(fn UpdateDraggedUnitLocation
  (bind _returnvalue (CallFunction|GetMovingUnit))
  (bind _returnvalue_2 (CallFunction|GetFocusedSquare))
  (bind _returnvalue_3 (Transformation|GetActorLocation _returnvalue))
  (Utilities|IsValid _returnvalue_2
    (:Is%20Valid
      (LocalVariables|SetsquareTempLoc (Transformation|GetActorLocation _returnvalue_2)))
    (:Is%20Not%20Valid
      (LocalVariables|SetsquareTempLoc (Variables|Default|GetFingerLocation))))
  (if (Variables|Default|GetbDragging)
    (if (Utilities|IsValid _returnvalue)
      (Transformation|SetActorLocation _returnvalue (Math|Interpolation|VInterpTo _returnvalue_3 (Math|Vector|MakeVector (.X (Math|Vector|BreakVector (select (Variables|Default|GetbSnapMove) (LocalVariables|GetsquareTempLoc) (Variables|Default|GetFingerLocation)))) (.Y (Math|Vector|BreakVector (select (Variables|Default|GetbSnapMove) (LocalVariables|GetsquareTempLoc) (Variables|Default|GetFingerLocation)))) (.Z (Math|Vector|BreakVector _returnvalue_3))) (Variables|Default|GetDragTriggerDelay) (Variables|Default|GetMoveSpeed)) false false))))

(fn StartHolding
  (Variables|Default|SetbHolding true))

(fn StopHolding
  (CallFunction|StopDragging)
  (Variables|Default|SetbHolding false))

(fn GetUnitinSquare
  (return (Variables|/Game/MergeProgress/Level/BP_Square.BP_Square_C|GetHostedUnit (CallFunction|GetFocusedSquare))))

(fn GetMovingUnit
  (return (Variables|Default|GetMovingUnit)))

(fn StartMerging
  (params (DroppedObject :type BP%20Pawn%20Object%20Reference) (MergingObject :type BP%20Pawn%20Object%20Reference))
  (if (and (Utilities|IsValid DroppedObject) (Utilities|IsValid MergingObject))
    (switch Utilities|FlowControl|Switch|SwitchonEElementMergeInstruction (Variables|/Game/MergeProgress/DataAssets/BP_ElementInfo.BP_ElementInfo_C|GetInstructions (Variables|/Game/MergeProgress/Mergeable_Object/BP_Pawn.BP_Pawn_C|GetInfo DroppedObject))
      (:NewEnumerator0
        (if (Variables|/Game/MergeProgress/DataAssets/BP_ElementInfo.BP_ElementInfo_C|GetbDiscovered (Variables|/Game/MergeProgress/Mergeable_Object/BP_Pawn.BP_Pawn_C|GetInfo DroppedObject))
          _
          (else
            (Variables|/Game/MergeProgress/DataAssets/BP_ElementInfo.BP_ElementInfo_C|SetbDiscovered (Variables|/Game/MergeProgress/Mergeable_Object/BP_Pawn.BP_Pawn_C|GetInfo DroppedObject) true)))
        (if (.ReturnValue (Utilities|Map|Find (Variables|/Game/MergeProgress/DataAssets/BP_ElementInfo.BP_ElementInfo_C|GetRecipes (Variables|/Game/MergeProgress/Mergeable_Object/BP_Pawn.BP_Pawn_C|GetInfo DroppedObject)) (Variables|/Game/MergeProgress/DataAssets/BP_ElementInfo.BP_ElementInfo_C|GetID (Variables|/Game/MergeProgress/Mergeable_Object/BP_Pawn.BP_Pawn_C|GetInfo MergingObject))))
          (Utilities|FlowControl|Sequence
            (:then_0
              (bind _returnvalue (Game|SpawnActorfromClass "/Game/MergeProgress/Mergeable_Object/BP_Pawn.BP_Pawn_C" (Math|Transform|MakeTransform (Transformation|GetWorldLocation (Variables|/Script/Engine.Actor|GetRootComponent MergingObject)) "0,45.000000, 0") "AlwaysSpawn" 0 0))
              (Utilities|FlowControl|Sequence
                (:then_0
                  (bind _returnvalue_2 (Components|StaticMesh|SetStaticMesh (Variables|/Game/MergeProgress/Mergeable_Object/BP_Pawn.BP_Pawn_C|GetCube _returnvalue) (Variables|/Game/MergeProgress/DataAssets/BP_ElementInfo.BP_ElementInfo_C|GetMesh (.Value (Utilities|Map|Find (Variables|/Game/MergeProgress/DataAssets/BP_ElementInfo.BP_ElementInfo_C|GetRecipes (Variables|/Game/MergeProgress/Mergeable_Object/BP_Pawn.BP_Pawn_C|GetInfo DroppedObject)) (Variables|/Game/MergeProgress/DataAssets/BP_ElementInfo.BP_ElementInfo_C|GetID (Variables|/Game/MergeProgress/Mergeable_Object/BP_Pawn.BP_Pawn_C|GetInfo MergingObject)))))))
                  (Development|PrintString "Error setting the static mesh after a merge" (not _returnvalue_2) (not _returnvalue_2) "(R=1.000000,G=0.000000,B=0.000000,A=1.000000)"))
                (:then_1
                  (bind _output_get (Variables|/Game/MergeProgress/Mergeable_Object/BP_Pawn.BP_Pawn_C|SetInfo _returnvalue (.Value (Utilities|Map|Find (Variables|/Game/MergeProgress/DataAssets/BP_ElementInfo.BP_ElementInfo_C|GetRecipes (Variables|/Game/MergeProgress/Mergeable_Object/BP_Pawn.BP_Pawn_C|GetInfo DroppedObject)) (Variables|/Game/MergeProgress/DataAssets/BP_ElementInfo.BP_ElementInfo_C|GetID (Variables|/Game/MergeProgress/Mergeable_Object/BP_Pawn.BP_Pawn_C|GetInfo MergingObject))))))
                  (CallFunction|CheckNewRenewable _output_get))))
            (:then_1
              (Actor|DestroyActor DroppedObject))
            (:then_2
              (Actor|DestroyActor MergingObject))
            (:then_3
              (CallFunction|MergeDone)))
          (else
            (Variables|/Game/MergeProgress/Level/BP_Square.BP_Square_C|SetHostedUnit (Variables|Default|GetInitialMovingSquare) (CallFunction|GetMovingUnit))
            (CallFunction|InvalidMove))))
      (:NewEnumerator1
        ;[1 1 1] TODO: Spawn feature elements
        (if (Variables|/Game/MergeProgress/DataAssets/BP_ElementInfo.BP_ElementInfo_C|GetbDiscovered (Variables|/Game/MergeProgress/Mergeable_Object/BP_Pawn.BP_Pawn_C|GetInfo DroppedObject))
          (CallFunction|InvalidMove :!label _label)
          (elif (Variables|/Game/MergeProgress/DataAssets/BP_ElementInfo.BP_ElementInfo_C|GetbReMergeable (Variables|/Game/MergeProgress/Mergeable_Object/BP_Pawn.BP_Pawn_C|GetInfo DroppedObject))
            (Variables|/Game/MergeProgress/DataAssets/BP_ElementInfo.BP_ElementInfo_C|SetbReMergeable (Variables|/Game/MergeProgress/Mergeable_Object/BP_Pawn.BP_Pawn_C|GetInfo DroppedObject) false)
            (Variables|/Game/MergeProgress/DataAssets/BP_ElementInfo.BP_ElementInfo_C|SetbDiscovered (Variables|/Game/MergeProgress/Mergeable_Object/BP_Pawn.BP_Pawn_C|GetInfo DroppedObject) false)
            (else
              (goto _label))))))))

(fn CheckNewRenewable
  (params (ElementInfo :type BP%20Element%20Info%20Object%20Reference))
  (bind _listrenewable (Variables|Default|GetLIstRenewable))
  (bind _returnvalue (Utilities|Array|FindItem _listrenewable ElementInfo))
  (bind _asbp_test_apple_spawner (Utilities|Casting|CastToBP_Test_AppleSpawner (Game|Player|GetPlayerPawn 0)))
  (Utilities|Array|SetArrayElem (Variables|/Game/MergeProgress/Spawner/BP_Test_AppleSpawner.BP_Test_AppleSpawner_C|GetSpawnNumber _asbp_test_apple_spawner) _returnvalue 0) ; Attivo il relativo bottone nell'HUD
  (Utilities|Time|UnpauseTimerbyHandle (Utilities|Array|Get(acopy) (Variables|/Game/MergeProgress/Spawner/BP_Test_AppleSpawner.BP_Test_AppleSpawner_C|Gettimeme _asbp_test_apple_spawner) _returnvalue)) ; Attivo il relativo Timer
)