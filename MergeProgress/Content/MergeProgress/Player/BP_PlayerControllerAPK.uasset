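; Touch player controller for a merge game: drags units between BP_Square tiles, tracks swipes, creates the gameplay HUD and spawns saved pending animals outside the city map.
; Each tick, finger traces set the focused square, which starts dragging its unit and interpolates it along.
; Drops move to free squares, merge via the unit's recipe map, or return.
; Map_Prototype_City disables merging and checks neighbouring squares for 2x2 placement.
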(event Custom|MergeDone
  (bind _returnvalue (CallFunction|GetFocusedSquare))
  ;[1 1 1] Merge has been executed on the chosen element
  (Utilities|IsValid _returnvalue
    (:Is%20Valid
      _)
    (:Is%20Not%20Valid
      (Default|SetFocused (Variables|Default|GetMovingUnit) false)))
  (Variables|Default|SetMovingUnit 0)
  (Variables|Default|SetbDragging false)
  (Variables|Default|SetbHolding false)
  (Variables|/Game/MergeProgress/Level/BP_Square.BP_Square_C|SetHostedUnit _returnvalue 0))

(event Custom|InvalidMove
  ;[1 1 1] InvalidMove
  (Variables|/Game/MergeProgress/Mergeable_Object/BP_Pawn.BP_Pawn_C|SetDragged (Variables|Default|GetMovingUnit) false)
  (if (Utilities|Enum|Equal(Enum) (Variables|Default|GetLevelName) "Map_Prototype_City")
    (Components|MoveComponentTo (Variables|/Script/Engine.Actor|GetRootComponent (Variables|Default|GetMovingUnit)) (+ (Transformation|GetActorLocation (Variables|/Game/MergeProgress/Mergeable_Object/BP_Pawn.BP_Pawn_C|GetInitialSquare (Variables|Default|GetMovingUnit))) "100.000000,-100.000000,10.000000") "-0.000000,90.000000,0.000000" true false (Variables|Default|GetFinalMoveDuration) false)
    (for _array_element (Variables|/Game/MergeProgress/Level/BP_Square.BP_Square_C|GetVicini_2*2 (Variables|/Game/MergeProgress/Mergeable_Object/BP_Pawn.BP_Pawn_C|GetInitialSquare (Variables|Default|GetMovingUnit)))
      (Variables|/Game/MergeProgress/Level/BP_Square.BP_Square_C|SetHostedUnit _array_element (Variables|Default|GetMovingUnit)))
    (else
      (Components|MoveComponentTo (Variables|/Script/Engine.Actor|GetRootComponent (Variables|Default|GetMovingUnit)) (+ (Transformation|GetActorLocation (Variables|Default|GetInitialMovingSquare)) "0, 0,10.000000") "0,90.000000, 0" true false (Variables|Default|GetFinalMoveDuration) false)))
  (Utilities|IsValid (CallFunction|GetFocusedSquare)
    (:Is%20Valid
      _)
    (:Is%20Not%20Valid
      (Default|SetFocused (Variables|Default|GetMovingUnit) false)))
  (Variables|Default|SetMovingUnit 0)
  (Variables|Default|SetbDragging false)
  (Variables|Default|SetbHolding false))

(event Custom|CanSaveAgain
  ;[1 1 1] Reset per poter salvare di nuovo
  (Variables|Default|SetCanSave false)
  (Utilities|FlowControl|RetriggerableDelay 1.0)
  (Variables|Default|SetCanSave true))

(event Custom|FinalStopMove
  (bind _lastfocusedsquare (Variables|Default|GetLastFocusedSquare))
  (bind _finalmoveduration (Variables|Default|GetFinalMoveDuration))
  (bind _lastfocusedsquare_2 (Variables|Default|GetLastFocusedSquare))
  (bind _returnvalue (Transformation|GetActorLocation _lastfocusedsquare_2))
  ;[1 1 1] Move element to selected square
  (if (Utilities|Enum|Equal(Enum) (Variables|Default|GetLevelName) "Map_Prototype_City")
    (Components|MoveComponentTo (Variables|/Script/Engine.Actor|GetRootComponent (Variables|Default|GetMovingUnit)) (+ _returnvalue "100.000000,-100.000000,10.000000") "-0.000000,90.000000,0.000000" true false _finalmoveduration false)
    (for _array_element (Variables|/Game/MergeProgress/Level/BP_Square.BP_Square_C|GetVicini_2*2 _lastfocusedsquare)
      (Variables|/Game/MergeProgress/Level/BP_Square.BP_Square_C|SetHostedUnit _array_element (Variables|Default|GetMovingUnit)))
    (Variables|/Game/MergeProgress/Mergeable_Object/BP_Pawn.BP_Pawn_C|SetInitialSquare (Variables|Default|GetMovingUnit) _lastfocusedsquare)
    (else
      (Components|MoveComponentTo (Variables|/Script/Engine.Actor|GetRootComponent (Variables|Default|GetMovingUnit)) (+ _returnvalue "0.000000, 0,10.000000") "0.000000,90.000000,0.000000" true false _finalmoveduration false)))
  (Utilities|IsValid (CallFunction|GetFocusedSquare)
    (:Is%20Valid
      _)
    (:Is%20Not%20Valid
      (Default|SetFocused (Variables|Default|GetMovingUnit) false)))
  (Variables|Default|SetMovingUnit 0)
  (Variables|Default|SetbDragging false)
  (Variables|Default|SetbHolding false)
  (Variables|Default|SetDropping true))

(event Custom|DragCoords
  (params (ScreenSpace :type Vector%202D%20Structure) (ActorPayload :type Actor%20Object%20Reference))
  (bind _pixelposition (Class|SlateBlueprintLibrary|AbsolutetoViewport ScreenSpace))
  (bind _self self)
  (bind (_worldposition _worlddirection) (Class|GameplayStatics|DeprojectScreentoWorld _self _pixelposition))
  (bind _outhit (Collision|LineTraceByChannel (Transformation|GetActorLocation (Game|GetPlayerCameraManager 0)) (+ _worldposition (* _worlddirection 5e+03)) "TraceTypeQuery1" true 0 "None"))
  (Transformation|SetActorLocation ActorPayload (.Location (Collision|BreakHitResult _outhit)) false false))

(event EventBeginPlay
  (bind _returnvalue (Game|GetCurrentLevelName true))
  (Variables|Default|SetLevelName _returnvalue)
  (bind _returnvalue_2 (UserInterface|CreateWidget "/Game/MergeProgress/HUD/HUD_Gameplay.HUD_Gameplay_C" (Game|GetPlayerController 0)))
  (bind _output_get (Variables|Default|SetHUDWidget _returnvalue_2))
  (UserInterface|Viewport|AddtoViewport _output_get 0)
  (CallFunction|SpawnfromArray))

(event EventTick
  (params (DeltaSeconds :type Float%20%28single-precision%29))
  (bind _returnvalue (Game|GetPlayerController 0))
  (bind (_locationx _locationy) (Class|PlayerController|GetInputTouchState _returnvalue "Touch1"))
  (bind _returnvalue_2 (Math|Vector2D|MakeVector2D _locationx _locationy))
  (|CallParentFunction DeltaSeconds)
  (CallFunction|FindFocusedSquare)
  (CallFunction|UpdateDraggedUnitLocation)
  (Utilities|FlowControl|Gate true
    (:Exit
      (if (not (Variables|Default|GetbDragging))
        (if (>= (Math|Vector2D|Vector2DLength (- _returnvalue_2 (stale Input|ActionEvents|InputActionFinger1 _output_get))) (Variables|Default|GetSwipeThreshold))
          (Variables|Default|SetStartLoc "(X=9999999980506447872.000000,Y=9999999980506447872.000000)")
          (Variables|Default|SetX (.y (* (- _returnvalue_2 (Variables|Default|GetPriorLoc)) (Variables|Default|GetSwipeSpeed))))
          (Variables|Default|SetY (.x (* (- _returnvalue_2 (Variables|Default|GetPriorLoc)) (Variables|Default|GetSwipeSpeed))))
          (Variables|Default|SetPriorLoc _returnvalue_2)
          (Variables|Default|SetSwiping true))))))

(event Input|ActionEvents|InputActionFinger1
  (params (Key :type Key%20Structure :default "None"))
  (bind _returnvalue (Game|GetPlayerController 0))
  (bind (_locationx _locationy) (Class|PlayerController|GetInputTouchState _returnvalue "Touch1"))
  (bind _returnvalue_2 (Math|Vector2D|MakeVector2D _locationx _locationy))
  (:Pressed
    (bind _output_get (Variables|Default|SetStartLoc _returnvalue_2))
    (Variables|Default|SetPriorLoc _output_get)
    (Utilities|FlowControl|Gate true) ; enters at Open
  )
  (:Released
    (Variables|Default|SetSwiping false)
    (Utilities|FlowControl|Gate true) ; enters at Close
  ))

(event Input|TouchEvents|InputTouch
  (params (Location :type Vector) (FingerIndex :type ETouchIndex%20Enum))
  ;[1 1 1] Drag'N'Drop logic
  (:Pressed
    (CallFunction|UnfocusSquare)
    (Variables|Default|SetbFocusing true))
  (:Released
    (Variables|Default|SetbFocusing false)
    (if (not (not (Variables|Default|GetbDragging)))
      (if (not (Variables|Default|GetbHolding))
        (CallFunction|StopHolding)
        (Variables|Default|SetbFocusing false)
        (Variables|Default|SetPressed false)))))

(fn ConstructionScript)

(fn FindFocusedSquare
  (if (not (Variables|Default|GetSwiping))
    (if (not (Variables|Default|GetisPinched))
      (if (Variables|Default|GetbFocusing)
        (bind _output_get (Variables|Default|SetFingerLocation (.ImpactPoint (Collision|BreakHitResult (.HitResult (Class|PlayerController|GetHitResultUnderFingerbyChannel "Touch1" "TraceTypeQuery1" (.bIsCurrentlyPressed (Class|PlayerController|GetInputTouchState (Variables|Default|GetFinger%20Index_0)))))))))
        (bind _outhits (Collision|MultiSphereTraceByChannel _output_get (+ _output_get "0, 0,50.000000") 1.0 "TraceTypeQuery4" false 0 "ForOneFrame"))
        (Utilities|IsValid (.HitActor (Collision|BreakHitResult (Utilities|Array|Get(acopy) _outhits)))
          (:Is%20Valid
            (bind _asbp_square (Utilities|Casting|CastToBP_Square (.HitActor (Collision|BreakHitResult (Utilities|Array|Get(acopy) _outhits))))
              (:then
                (if (!= _asbp_square (Variables|Default|GetFocusedSquare))
                  (CallFunction|UnfocusSquare)
                  (CallFunction|SetFocusedSquare _asbp_square)
                  (else
                    (Rendering|Debug|DrawDebugPoint (Transformation|GetActorLocation _asbp_square) 1e+01 "(R=1.000000,G=0.402425,B=0.000000,A=1.000000)" 0.0))))
              (:CastFailed
                (CallFunction|UnfocusSquare :!label _label))))
          (:Is%20Not%20Valid
            (goto _label)))))))

(fn SetFocusedSquare
  (params (Square :type BP%20Square%20Object%20Reference))
  (Variables|Default|SetFocusedSquare Square)
  (if (not (Variables|Default|GetbDragging))
    (Utilities|IsThereUnitinFocusedSquare
      (:Valid
        (Default|SetFocused (CallFunction|GetUnitinSquare) true)
        (CallFunction|StartDragging)))))

(fn UnfocusSquare
  (Utilities|IsValid (CallFunction|GetFocusedSquare)
    (:Is%20Valid
      (if (not (Variables|Default|GetbDragging))
        (Utilities|IsThereUnitinFocusedSquare
          (:Valid
            (Default|SetFocused (CallFunction|GetUnitinSquare) false))
          (:Invalid
            _))))
    (:Is%20Not%20Valid
      _))
  (Utilities|IsValid (Variables|Default|GetFocusedSquare)
    (:Is%20Valid
      (Variables|Default|SetLastFocusedSquare (Variables|Default|GetFocusedSquare)))
    (:Is%20Not%20Valid
      _))
  (Variables|Default|SetFocusedSquare 0))

(fn GetFocusedSquare
  (return (Variables|Default|GetFocusedSquare)))

(fn StartDragging
  (bind _returnvalue (CallFunction|GetUnitinSquare))
  (bind _returnvalue_2 (CallFunction|GetFocusedSquare))
  (bind _info (Variables|/Game/MergeProgress/Mergeable_Object/BP_Pawn.BP_Pawn_C|GetInfo _returnvalue))
  (if (not (or (Utilities|Set|Contains (Variables|Default|GetNeutriList) _info) (Utilities|Enum|Equal(Enum) (Variables|/Game/MergeProgress/DataAssets/Animals_DataAssets/BP_ElementInfo.BP_ElementInfo_C|GetID _info) "")))
    (Variables|Default|SetMovingUnit _returnvalue)
    (Variables|Default|SetbDragging true)
    (Default|SetDragState (CallFunction|GetMovingUnit) true)
    (Variables|Default|SetInitialMovingSquare _returnvalue_2)
    (Variables|/Game/MergeProgress/Level/BP_Square.BP_Square_C|SetHostedUnit _returnvalue_2 (Variables|Default|GetHosted%20Unit))
    (if (Utilities|Enum|Equal(Enum) (Variables|Default|GetLevelName) "Map_Prototype_City")
      (bind _outactors (Actor|GetAllActorsOfClass "/Game/MergeProgress/Level/BP_Square.BP_Square_C"))
      (for _array_element _outactors
        (if (== (Variables|/Game/MergeProgress/Level/BP_Square.BP_Square_C|GetHostedUnit _array_element) (CallFunction|GetMovingUnit))
          (Variables|/Game/MergeProgress/Level/BP_Square.BP_Square_C|SetHostedUnit _array_element 0)))
      (else
        (bind _outactors_2 (Actor|GetAllActorsOfClass "/Game/MergeProgress/Level/BP_Pilastro.BP_Pilastro_C"))
        (for _array_element_2 _outactors_2
          (Default|SpawnNeutro _array_element_2))))))

(fn StopDragging
  (bind _returnvalue (CallFunction|GetFocusedSquare))
  (bind _returnvalue_2 (CallFunction|GetFocusedSquare))
  (bind _returnvalue_3 (CallFunction|GetMovingUnit))
  (bind _returnvalue_4 (CallFunction|GetMovingUnit))
  (bind _returnvalue_5 (Utilities|GetClass _returnvalue))
  (CallFunction|CanSaveAgain)
  (Utilities|IsValid _returnvalue_2
    (:Is%20Valid
      (Variables|Default|SetLastFocusedSquare _returnvalue_2)
      (Utilities|IsThereUnitinFocusedSquare
        (:Valid
          (if (Utilities|IsValid (CallFunction|GetUnitinSquare))
            (if (Utilities|Enum|Equal(Enum) (Variables|Default|GetLevelName) "Map_Prototype_City")
              (Default|SetDragState (CallFunction|GetMovingUnit) false :!label _label)
              (if (Utilities|Enum|Equal(Enum) (Variables|Default|GetLevelName) "Map_Prototype_City")
                (Variables|/Game/MergeProgress/Level/BP_Square.BP_Square_C|SetHostedUnit (Variables|/Game/MergeProgress/Mergeable_Object/BP_Pawn.BP_Pawn_C|GetInitialSquare _returnvalue_4) _returnvalue_4)
                (else
                  (Variables|/Game/MergeProgress/Level/BP_Square.BP_Square_C|SetHostedUnit (Variables|Default|GetInitialMovingSquare) _returnvalue_4)))
              (CallFunction|InvalidMove)
              (else
                (CallFunction|StartMerging (CallFunction|GetMovingUnit) (CallFunction|GetUnitinSquare))))
            (else
              (goto _label))))
        (:Invalid
          (bind _asmy_game_instance (Utilities|Casting|CastToMyGameInstance (Game|GetGameInstance)))
          (if (or (== _returnvalue_5 "/Game/MergeProgress/Level/BP_Square.BP_Square_C") (== _returnvalue_5 "/Game/MergeProgress/Level/BP_Pilastro.BP_Pilastro_C"))
            _
            (elif (<= (Variables|/Game/MergeProgress/GameInstance/SaveGameObject.SaveGameObject_C|GetNumberAnimalsBoat (Variables|/Game/MergeProgress/GameInstance/MyGameInstance.MyGameInstance_C|GetSaveGameData _asmy_game_instance)) 15)
              _
              (else
                (goto _label))))
          (if (Utilities|Enum|Equal(Enum) (Variables|Default|GetLevelName) "Map_Prototype_City")
            (|CheckSquareVicini
              (:then
                (goto _label))
              (:then2
                (goto _label))
              (:then3
                (goto _label))
              (:then4
                (goto _label))
              (:else
                _)))
          (Default|SetDragState _returnvalue_3 false)
          (Variables|/Game/MergeProgress/Level/BP_Square.BP_Square_C|SetHostedUnit (Variables|Default|GetLastFocusedSquare) _returnvalue_3)
          (CallFunction|FinalStopMove))))
    (:Is%20Not%20Valid
      (goto _label))))

(fn UpdateDraggedUnitLocation
  (bind _returnvalue (CallFunction|GetMovingUnit))
  (bind _returnvalue_2 (CallFunction|GetFocusedSquare))
  (bind _returnvalue_3 (Transformation|GetActorLocation _returnvalue))
  (Utilities|IsValid _returnvalue_2
    (:Is%20Valid
      (LocalVariables|SetsquareTempLoc (Transformation|GetActorLocation _returnvalue_2)))
    (:Is%20Not%20Valid
      (LocalVariables|SetsquareTempLoc (Variables|Default|GetFingerLocation))))
  (if (Variables|Default|GetbDragging)
    (if (Utilities|IsValid _returnvalue)
      (if (== (Variables|/Game/MergeProgress/Mergeable_Object/BP_Pawn.BP_Pawn_C|GetInfo_Building _returnvalue) 0)
        (Transformation|SetActorLocation _returnvalue (Math|Interpolation|VInterpTo _returnvalue_3 (Math|Vector|MakeVector (.X (Math|Vector|BreakVector (select (Variables|Default|GetbSnapMove) (LocalVariables|GetsquareTempLoc) (Variables|Default|GetFingerLocation)))) (.Y (Math|Vector|BreakVector (select (Variables|Default|GetbSnapMove) (LocalVariables|GetsquareTempLoc) (Variables|Default|GetFingerLocation)))) (.Z (Math|Vector|BreakVector _returnvalue_3))) (Variables|Default|GetDragTriggerDelay) (Variables|Default|GetMoveSpeed)) false false)
        (else
          (Transformation|SetActorLocation _returnvalue (+ (Math|Interpolation|VInterpTo _returnvalue_3 (Math|Vector|MakeVector (.X (Math|Vector|BreakVector (select (Variables|Default|GetbSnapMove) (LocalVariables|GetsquareTempLoc) (Variables|Default|GetFingerLocation)))) (.Y (Math|Vector|BreakVector (select (Variables|Default|GetbSnapMove) (LocalVariables|GetsquareTempLoc) (Variables|Default|GetFingerLocation)))) (.Z (Math|Vector|BreakVector _returnvalue_3))) (Variables|Default|GetDragTriggerDelay) (Variables|Default|GetMoveSpeed)) "100.000000,-100.000000, 0") false false))))))

(fn StartHolding
  (Variables|Default|SetbHolding true))

(fn StopHolding
  (CallFunction|StopDragging)
  (Variables|Default|SetbHolding false))

(fn GetUnitinSquare
  (return (Variables|/Game/MergeProgress/Level/BP_Square.BP_Square_C|GetHostedUnit (CallFunction|GetFocusedSquare))))

(fn GetMovingUnit
  (return (Variables|Default|GetMovingUnit)))

(fn StartMerging
  (params (DroppedObject :type BP%20Pawn%20Object%20Reference) (MergingObject :type BP%20Pawn%20Object%20Reference))
  (if (and (Utilities|IsValid DroppedObject) (Utilities|IsValid MergingObject))
    (if (Variables|/Game/MergeProgress/DataAssets/Animals_DataAssets/BP_ElementInfo.BP_ElementInfo_C|GetbDiscovered (Variables|/Game/MergeProgress/Mergeable_Object/BP_Pawn.BP_Pawn_C|GetInfo DroppedObject))
      _
      (else
        (Variables|/Game/MergeProgress/DataAssets/Animals_DataAssets/BP_ElementInfo.BP_ElementInfo_C|SetbDiscovered (Variables|/Game/MergeProgress/Mergeable_Object/BP_Pawn.BP_Pawn_C|GetInfo DroppedObject) true)))
    (if (.ReturnValue (Utilities|Map|Find (Variables|/Game/MergeProgress/DataAssets/Animals_DataAssets/BP_ElementInfo.BP_ElementInfo_C|GetRecipes (Variables|/Game/MergeProgress/Mergeable_Object/BP_Pawn.BP_Pawn_C|GetInfo DroppedObject)) (Variables|/Game/MergeProgress/DataAssets/Animals_DataAssets/BP_ElementInfo.BP_ElementInfo_C|GetID (Variables|/Game/MergeProgress/Mergeable_Object/BP_Pawn.BP_Pawn_C|GetInfo MergingObject))))
      (CallFunction|CanSaveAgain)
      (Utilities|FlowControl|Sequence
        (:then_0
          (bind _returnvalue (Game|SpawnActorfromClass "/Game/MergeProgress/Mergeable_Object/BP_Pawn.BP_Pawn_C" (Math|Transform|MakeTransform (Transformation|GetWorldLocation (Variables|/Script/Engine.Actor|GetRootComponent (Variables|Default|GetFocusedSquare))) "0,90.000000,0.000000") "AlwaysSpawn" 0 0))
          (bind _output_get (Variables|/Game/MergeProgress/Mergeable_Object/BP_Pawn.BP_Pawn_C|SetInfo _returnvalue (.Value (Utilities|Map|Find (Variables|/Game/MergeProgress/DataAssets/Animals_DataAssets/BP_ElementInfo.BP_ElementInfo_C|GetRecipes (Variables|/Game/MergeProgress/Mergeable_Object/BP_Pawn.BP_Pawn_C|GetInfo DroppedObject)) (Variables|/Game/MergeProgress/DataAssets/Animals_DataAssets/BP_ElementInfo.BP_ElementInfo_C|GetID (Variables|/Game/MergeProgress/Mergeable_Object/BP_Pawn.BP_Pawn_C|GetInfo MergingObject))))))
          (Default|Birth _returnvalue)
          (CallFunction|CheckNewRenewable _output_get)
          (Default|SendtoCity (Variables|Default|GetHUDWidget) false _output_get))
        (:then_1
          (Actor|DestroyActor DroppedObject))
        (:then_2
          (Actor|DestroyActor MergingObject))
        (:then_3
          (CallFunction|MergeDone)))
      (else
        (Variables|/Game/MergeProgress/Level/BP_Square.BP_Square_C|SetHostedUnit (Variables|Default|GetInitialMovingSquare) (CallFunction|GetMovingUnit))
        (CallFunction|InvalidMove)))))

(fn CheckNewRenewable
  (params (ElementInfo :type BP%20Element%20Info%20Object%20Reference))
  (bind _listrenewable (Variables|Default|GetLIstRenewable))
  (bind _returnvalue (Utilities|Array|FindItem _listrenewable ElementInfo))
  ;[1 1 1] Da Rivedere la Logica di Spawning
  (bind _asbp_test_apple_spawner (Utilities|Casting|CastToBP_Test_AppleSpawner (Game|Player|GetPlayerPawn 0)))
  (Utilities|Array|SetArrayElem (Variables|/Game/MergeProgress/Spawner/BP_Test_AppleSpawner.BP_Test_AppleSpawner_C|GetSpawnNumber _asbp_test_apple_spawner) _returnvalue 0) ; Attivo il relativo bottone nell'HUD
  (Utilities|Time|UnpauseTimerbyHandle (Utilities|Array|Get(acopy) (Variables|/Game/MergeProgress/Spawner/BP_Test_AppleSpawner.BP_Test_AppleSpawner_C|Gettimeme _asbp_test_apple_spawner) _returnvalue)) ; Attivo il relativo Timer
)

(fn SpawnfromArray
  (bind _returnvalue (Game|GetCurrentLevelName true))
  (if (not (Utilities|Enum|Equal(Enum) _returnvalue "Map_Prototype_City"))
    (bind _asmy_game_instance (Utilities|Casting|CastToMyGameInstance (Game|GetGameInstance)))
    (bind _outactors (Actor|GetAllActorsOfClass "/Game/MergeProgress/Level/BP_Square.BP_Square_C"))
    (for _index (range 0 (Utilities|Array|Length (Variables|/Game/MergeProgress/GameInstance/SaveGameObject.SaveGameObject_C|GetAnimalsToSpawn (Variables|/Game/MergeProgress/GameInstance/MyGameInstance.MyGameInstance_C|GetSaveGameData _asmy_game_instance))))
      (bind _asmy_game_instance_2 (Utilities|Casting|CastToMyGameInstance (Game|GetGameInstance)))
      (bind _array_element (Utilities|Array|ForEachLoopwithBreak _outactors)
        (:LoopBody
          (if (Math|Boolean|ANDBoolean (not (== (Utilities|GetClass _array_element) "/Game/MergeProgress/Level/BP_Pilastro.BP_Pilastro_C")) (!= (Utilities|Array|Get(acopy) (Variables|/Game/MergeProgress/GameInstance/SaveGameObject.SaveGameObject_C|GetAnimalsToSpawn (Variables|/Game/MergeProgress/GameInstance/MyGameInstance.MyGameInstance_C|GetSaveGameData _asmy_game_instance_2)) (Utilities|Array|LastIndex (Variables|/Game/MergeProgress/GameInstance/SaveGameObject.SaveGameObject_C|GetAnimalsToSpawn (Variables|/Game/MergeProgress/GameInstance/MyGameInstance.MyGameInstance_C|GetSaveGameData _asmy_game_instance_2)))) 0) (not (Utilities|Set|Contains (Variables|Default|GetNeutriList) (Utilities|Array|Get(acopy) (Variables|/Game/MergeProgress/GameInstance/SaveGameObject.SaveGameObject_C|GetAnimalsToSpawn (Variables|/Game/MergeProgress/GameInstance/MyGameInstance.MyGameInstance_C|GetSaveGameData _asmy_game_instance_2)) (Utilities|Array|LastIndex (Variables|/Game/MergeProgress/GameInstance/SaveGameObject.SaveGameObject_C|GetAnimalsToSpawn (Variables|/Game/MergeProgress/GameInstance/MyGameInstance.MyGameInstance_C|GetSaveGameData _asmy_game_instance_2)))))))
            (bind _asbp_square (Utilities|Casting|CastToBP_Square _array_element))
            (if (not (!= (Variables|/Game/MergeProgress/Level/BP_Square.BP_Square_C|GetHostedUnit _asbp_square) 0))
              (Default|SpawningObject (Variables|Default|GetSpawnerReference) (Utilities|Array|Get(acopy) (Variables|/Game/MergeProgress/GameInstance/SaveGameObject.SaveGameObject_C|GetAnimalsToSpawn (Variables|/Game/MergeProgress/GameInstance/MyGameInstance.MyGameInstance_C|GetSaveGameData _asmy_game_instance_2)) (Utilities|Array|LastIndex (Variables|/Game/MergeProgress/GameInstance/SaveGameObject.SaveGameObject_C|GetAnimalsToSpawn (Variables|/Game/MergeProgress/GameInstance/MyGameInstance.MyGameInstance_C|GetSaveGameData _asmy_game_instance_2)))) _asbp_square)
              (Utilities|Array|RemoveIndex (Variables|/Game/MergeProgress/GameInstance/SaveGameObject.SaveGameObject_C|GetAnimalsToSpawn (Variables|/Game/MergeProgress/GameInstance/MyGameInstance.MyGameInstance_C|GetSaveGameData _asmy_game_instance_2)) (Utilities|Array|LastIndex (Variables|/Game/MergeProgress/GameInstance/SaveGameObject.SaveGameObject_C|GetAnimalsToSpawn (Variables|/Game/MergeProgress/GameInstance/MyGameInstance.MyGameInstance_C|GetSaveGameData _asmy_game_instance_2)))))))))))